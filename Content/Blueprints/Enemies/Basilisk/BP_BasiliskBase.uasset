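; Base Basilisk enemy with melee bite, ranged venom spit and stunning grapple attacks, plus health and death.
; BeginPlay scales health and damage by a multiplier, and Rotate faces the player.
; DoOnce gates and delays pace attacks: sphere traces trigger bite and grapple damage, while Shoot passes damage to the spawned spit via ApplyDamage.
; Tick watches health, then disables attacks, plays audio and destroys the actor.
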(event Custom|Shoot
  ;[0.15 0.15 0.15 0.5] Range Attack Event with spawning web and reload
  (Utilities|FlowControl|DoOnce false :!label _label
    (:Completed
      (Development|PrintString "BasiliskrRangeAttack")
      (Variables|Default|SetCanShoot false)
      (bind _returnvalue (Game|SpawnActorfromClass "/Game/Blueprints/Enemies/Basilisk/BP_VenomSpit.BP_VenomSpit_C" (Transformation|GetWorldTransform (Variables|Default|GetArrow1)) "AlwaysSpawn" "MultiplyWithRoot" 0 0))
      (Game|Damage|ApplyDamage _returnvalue (Variables|Default|GetRangeAttackDamage) 0 self)
      (Utilities|FlowControl|Delay (Variables|Default|GetRangedAttackSpeed))
      (Variables|Default|SetCanShoot true)
      (goto _label Reset))))

(event Custom|Attack
  (bind _arrow1 (Variables|Default|GetArrow1))
  (bind _returnvalue (Transformation|GetWorldLocation _arrow1))
  ;[0.15 0.15 0.15 0.5] Melee Attack  with CoolDown
  (Utilities|FlowControl|DoOnce false :!label _label
    (:Completed
      (bind _returnvalue_2 (Collision|SphereTraceForObjects _returnvalue _returnvalue (Variables|Default|GetMeleeAttackRange) (Utilities|Array|MakeArray "ObjectTypeQuery7") false 0 "ForDuration"))
      (if _returnvalue_2
        (Variables|Default|SetCanBite false)
        (Development|PrintString "BasiliskMeleeAttack")
        (Game|Damage|ApplyDamage (Game|GetPlayerCharacter 0) (Variables|Default|GetMeleeAttackDamage) 0 0))
      (Utilities|FlowControl|Delay (Variables|Default|GetMeleeAttackSpeed))
      (Variables|Default|SetCanBite true)
      (goto _label Reset))))

(event Custom|Rotate
  ;[0.15 0.15 0.15 0.5] Ratating actor toward player
  (Transformation|SetActorRotation (Math|Rotator|FindLookatRotation (Transformation|GetActorLocation) (Transformation|GetActorLocation (Game|GetPlayerCharacter 0)))))

(event Custom|Grapple
  (bind _arrow1 (Variables|Default|GetArrow1))
  (bind _returnvalue (Transformation|GetWorldLocation _arrow1))
  ;[0.15 0.15 0.15 0.5] Grapple action and reload
  (Utilities|FlowControl|DoOnce false :!label _label
    (:Completed
      (bind _returnvalue_2 (Collision|SphereTraceForObjects _returnvalue _returnvalue (Variables|Default|GetGrappleAttackRange) (Utilities|Array|MakeArray "ObjectTypeQuery7") false 0 "ForDuration"))
      (if _returnvalue_2
        (Development|PrintString "BasiliskGrapple")
        (Variables|Default|SetCanGrapple false)
        (Game|Damage|ApplyDamage (Game|GetPlayerCharacter 0) (Variables|Default|GetGrappleAttackDamage) 0 0 "/Game/Blueprints/Combat/BP_StunDamageType.BP_StunDamageType_C")
        (Utilities|FlowControl|Delay (Variables|Default|GetGrappleAttackSpeed))
        (Variables|Default|SetCanGrapple true)
        (goto _label Reset)))))

(event EventBeginPlay
  ;[0.15 0.15 0.15 0.5] PresetVariables
  (Variables|Default|SetMaxHealth (* (Variables|Default|GetMaxHealth) (Variables|Default|GetMultipler)))
  (Variables|Default|SetCurrentHealth (Variables|Default|GetMaxHealth))
  (Variables|/Script/Engine.CharacterMovementComponent|SetMaxWalkSpeed (Variables|Character|GetCharacterMovement) (Variables|Default|GetMovementSpeed))
  (Variables|Default|SetMeleeAttackDamage (* (Variables|Default|GetMeleeAttackDamage) (Variables|Default|GetMultipler)))
  (Variables|Default|SetRangeAttackDamage (* (Variables|Default|GetRangeAttackDamage) (Variables|Default|GetMultipler)))
  (Variables|Default|SetGrappleAttackDamage (* (Variables|Default|GetGrappleAttackDamage) (Variables|Default|GetMultipler))))

(event Game|Damage|EventAnyDamage
  (params (Damage :type Float%20%28single-precision%29) (DamageType :type Damage%20Type%20Object%20Reference) (InstigatedBy :type Controller%20Object%20Reference) (DamageCauser :type Actor%20Object%20Reference))
  ;[0.15 0.15 0.15 0.5] Recieve Damage
  (Variables|Default|SetCurrentHealth (- (Variables|Default|GetCurrentHealth) Damage)))

(event EventTick
  (params (DeltaSeconds :type Float%20%28single-precision%29))
  (bind _basiliskaudio (Variables|Default|GetBasiliskAudio))
  ;[0.15 0.15 0.15 0.5] Death
  (if (<= (Variables|Default|GetCurrentHealth) 0.0)
    (Variables|Default|SetCanShoot false)
    (Variables|Default|SetCanBite false)
    (Variables|Default|SetCanGrapple false)
    (Utilities|FlowControl|DoOnce false
      (:Completed
        (Components|Movement|StopMovementImmediately (Variables|Character|GetCharacterMovement))
        (Audio|Components|Audio|SetVolumeMultiplier _basiliskaudio 0.5 :!class /Script/Engine.AudioComponent)
        (Audio|Components|Audio|Play _basiliskaudio 0.0)
        (Utilities|FlowControl|Delay 1.0)
        (Actor|DestroyActor)))))

(fn ConstructionScript)