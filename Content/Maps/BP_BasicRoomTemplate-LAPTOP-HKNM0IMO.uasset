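; BP_BasicRoomTemplate is a room template with four directional exit triggers that send the player on to the next level.
; Each trigger stores the world location and rotation of the opposite side's spawn component as the player's spawn transform, so a north exit leads to a south entry.
; If LevelBeaten is set, it then calls LoadNextLevel on BP_MainGameInstance with that transform and itself as the current level.
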(event OnComponentBeginOverlap(EastSpawnCollider)
  (params (OverlappedComponent :type Primitive%20Component%20Object%20Reference) (OtherActor :type Actor%20Object%20Reference) (OtherComp :type Primitive%20Component%20Object%20Reference) (OtherBodyIndex :type Integer) (bFromSweep :type Boolean) (SweepResult :type Hit%20Result%20Structure%20%28by%20ref%29))
  (Development|PrintString "ToWest" true true "(R=0.000000,G=1.000000,B=0.178313,A=1.000000)")
  (CallFunction|TransformPlayerPos (Variables|Default|GetWestSpawnVector))
  (if (Variables|Default|GetLevelBeaten)
    (bind _asbp_main_game_instance (Utilities|Casting|CastToBP_MainGameInstance (Game|GetGameInstance)))
    (Default|LoadNextLevel _asbp_main_game_instance (Variables|Default|GetPlayerSpawnVector) (Variables|Default|GetPlayerSpawnRot) self)))

(event OnComponentBeginOverlap(NorthSpawnCollider)
  (params (OverlappedComponent :type Primitive%20Component%20Object%20Reference) (OtherActor :type Actor%20Object%20Reference) (OtherComp :type Primitive%20Component%20Object%20Reference) (OtherBodyIndex :type Integer) (bFromSweep :type Boolean) (SweepResult :type Hit%20Result%20Structure%20%28by%20ref%29))
  (Development|PrintString "ToSouth")
  (CallFunction|TransformPlayerPos (Variables|Default|GetSouthSpawnVector))
  (if (Variables|Default|GetLevelBeaten)
    (bind _asbp_main_game_instance (Utilities|Casting|CastToBP_MainGameInstance (Game|GetGameInstance)))
    (Default|LoadNextLevel _asbp_main_game_instance (Variables|Default|GetPlayerSpawnVector) (Variables|Default|GetPlayerSpawnRot) self)))

(event OnComponentBeginOverlap(SouthSpawnCollider)
  (params (OverlappedComponent :type Primitive%20Component%20Object%20Reference) (OtherActor :type Actor%20Object%20Reference) (OtherComp :type Primitive%20Component%20Object%20Reference) (OtherBodyIndex :type Integer) (bFromSweep :type Boolean) (SweepResult :type Hit%20Result%20Structure%20%28by%20ref%29))
  (Development|PrintString "ToNorth" true true "(R=1.000000,G=0.118920,B=0.000000,A=1.000000)")
  (CallFunction|TransformPlayerPos (Variables|Default|GetNorthSpawnVector))
  (if (Variables|Default|GetLevelBeaten)
    (bind _asbp_main_game_instance (Utilities|Casting|CastToBP_MainGameInstance (Game|GetGameInstance)))
    (Default|LoadNextLevel _asbp_main_game_instance (Variables|Default|GetPlayerSpawnVector) (Variables|Default|GetPlayerSpawnRot) self)))

(event OnComponentBeginOverlap(WestSpawnCollider)
  (params (OverlappedComponent :type Primitive%20Component%20Object%20Reference) (OtherActor :type Actor%20Object%20Reference) (OtherComp :type Primitive%20Component%20Object%20Reference) (OtherBodyIndex :type Integer) (bFromSweep :type Boolean) (SweepResult :type Hit%20Result%20Structure%20%28by%20ref%29))
  (Development|PrintString "ToEast" true true "(R=1.000000,G=0.838396,B=0.000000,A=1.000000)")
  (CallFunction|TransformPlayerPos (Variables|Default|GetEastSpawnVector))
  (if (Variables|Default|GetLevelBeaten)
    (bind _asbp_main_game_instance (Utilities|Casting|CastToBP_MainGameInstance (Game|GetGameInstance)))
    (Default|LoadNextLevel _asbp_main_game_instance (Variables|Default|GetPlayerSpawnVector) (Variables|Default|GetPlayerSpawnRot) self)))

(fn ConstructionScript)

(fn TransformPlayerPos
  (params (Target :type Capsule%20Component%20Object%20Reference))
  (Variables|Default|SetPlayerSpawnVector (Transformation|GetWorldLocation Target))
  (Variables|Default|SetPlayerSpawnRot (Transformation|GetWorldRotation Target))
  (return))