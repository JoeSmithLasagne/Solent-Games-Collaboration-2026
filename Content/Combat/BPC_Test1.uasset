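; Test combat ability component that registers itself with its owner's instigator controller on BeginPlay.
; M1 sends the combat controller a short-lived, damaging hitbox just in front of the owner, keyed by component name plus an attack suffix and skipped if that key already returns a hitbox.
; M2 is empty; its wider hitbox logic and the component-removal notification sit in unconnected nodes that never run.
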(event EventBeginPlay
  (bind _returnvalue (Components|GetOwner))
  (bind _instigator (Variables|/Script/Engine.Actor|GetInstigator _returnvalue))
  (bind _returnvalue_2 (Pawn|GetController _instigator))
  (Class|BPICombatInterface|OnComponentAdded(Message) _returnvalue_2 self)
  (Development|PrintString (Utilities|GetDisplayName _returnvalue_2)))

(event EventM1
  (params (CombatController :type Actor%20Component%20Object%20Reference))
  (bind _self self)
  (bind _returnvalue (Utilities|GetDisplayName _self))
  (bind _returnvalue_2 (Components|GetOwner _self))
  (bind _returnvalue_3 (Transformation|GetActorTransform _returnvalue_2))
  (bind _returnvalue_4 (Utilities|String|Append _returnvalue "_M1"))
  (bind _returned (CallFunction|GetHitboxfromKey 0 _returnvalue_4))
  (if (not _returned)
    (Development|PrintString "1m out" false)
    (Class|BPICombatInterface|AddHitboxtoCombatController(Message) CombatController (Utilities|Struct|MakeStruct_HitboxData 0.1 2e+01 (Math|Transform|MakeTransform (+ (.location _returnvalue_3) (* (Math|Vector|GetForwardVector (.rotation _returnvalue_3)) 5e+01)) (.rotation _returnvalue_3) "100.000000,100.000000,100.000000") (Utilities|Time|GetGameTimeinSeconds) true _returnvalue_4))))

(event EventM2
  (params (CombatController :type Actor%20Component%20Object%20Reference)))