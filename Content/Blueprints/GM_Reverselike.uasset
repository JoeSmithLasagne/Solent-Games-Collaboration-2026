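; Game mode for Reverselike that provides RH_ helper functions to summon creatures and toggle the mouse cursor.
; RH_Summon maps a creature name to its pawn class and behavior tree, then spawns the requested count at random reachable points around the player or cursor.
; Cursor placement uses a visibility trace from the player camera toward the deprojected mouse, keeping the hit's X and Y at the player's height.
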(event EventBeginPlay)

(event EventTick
  (params (DeltaSeconds :type Float%20%28single-precision%29)))

(fn ConstructionScript)

(fn RHSummon
  (params (NameOfCreature :type Name) (Quantity :type Integer) (onMe%28Player%29/onMouse :type String) (SpawnRadius%281-inf%29 :type Float%20%28double-precision%29))
  (bind _returnvalue (Game|GetPlayerCharacter 0))
  (bind _returnvalue_2 (Transformation|GetActorLocation _returnvalue))
  (bind (_class _behaviourtree) (CallFunction|FindMobbyName NameOfCreature))
  (bind _output_get (LocalVariables|SetAmount Quantity))
  (while (> _output_get 0)
    (LocalVariables|SetAmount (- (LocalVariables|GetAmount) 1))
    (switch string onMe%28Player%29/onMouse
      (:Default
        (AI|SpawnAIFromClass _class _behaviourtree (.RandomLocation (AI|Navigation|GetRandomReachablePointinRadius (Math|Vector|MakeVector (.x _returnvalue_2) (.y _returnvalue_2) (.z _returnvalue_2)) SpawnRadius%281-inf%29 0 0)) "0, 0, 0" true 0 :!label _label))
      (:onMe
        (goto _label))
      (:onMouse
        (bind _mousevectorflatlocation (CallFunction|FindMouseFlatPosition))
        (AI|SpawnAIFromClass _class _behaviourtree (.RandomLocation (AI|Navigation|GetRandomReachablePointinRadius (Math|Vector|MakeVector (.x _mousevectorflatlocation) (.y _mousevectorflatlocation) (.z _returnvalue_2)) SpawnRadius%281-inf%29 0 0)) "0, 0, 0" true 0)))))

(fn FindMobbyName
  (params (Name :type Name))
  (switch name Name
    (:Spider
      (return (LocalVariables|GetSpider) (LocalVariables|GetSpiderBT)))
    (:Basilisk
      (return (LocalVariables|GetBasilisk) (LocalVariables|GetBasiliskBT)))
    (:Chimera
      (return (LocalVariables|GetChimera) (LocalVariables|GetChimeraBT)))
    (:SkeletonShield
      (return (LocalVariables|GetSkeleton) (LocalVariables|GetSkeletonBT)))
    (:Gnome
      (return (LocalVariables|GetGnome) (LocalVariables|GetGnomeBT)))
    (:Hydra
      (return (LocalVariables|GetHydra) (LocalVariables|GetHydraBT)))
    (:PosessedArmour
      (return (LocalVariables|GetPosessedArmour) (LocalVariables|GetPosessedArmourBT)))
    (:Harpy
      (return (LocalVariables|GetHarpy) (LocalVariables|GetHarpyBT)))))

(fn RHShowMouse
  (params (Show :type Boolean))
  (if Show
    (CallFunction|ShowMouse)
    (else
      (CallFunction|HideMouse))))

(fn FindMouseFlatPosition
  (bind _asbp_player_character (Utilities|Casting|CastToBP_PlayerCharacter (Game|GetPlayerCharacter 0)))
  (bind _outhit (Collision|LineTraceByChannel (Transformation|GetWorldLocation (Variables|/Game/Blueprints/BP_PlayerCharacter.BP_PlayerCharacter_C|GetCamera _asbp_player_character)) (* (+ (- (.WorldLocation (Game|Player|ConvertMouseLocationToWorldSpace (Game|GetPlayerController 0))) (Transformation|GetWorldLocation (Variables|/Game/Blueprints/BP_PlayerCharacter.BP_PlayerCharacter_C|GetCamera _asbp_player_character))) (Math|Vector|RotateVector (Math|Vector|GetForwardVector (Variables|/Game/Blueprints/BP_PlayerCharacter.BP_PlayerCharacter_C|GetCamera _asbp_player_character)) "40.000000,45.000000,0.000000")) 1e+03) "TraceTypeQuery1" false 0 "None"))
  (return (.Location (Collision|BreakHitResult _outhit))))