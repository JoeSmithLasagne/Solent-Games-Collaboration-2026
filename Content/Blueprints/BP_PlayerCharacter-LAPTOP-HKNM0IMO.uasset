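; Player character Blueprint handling camera-relative Enhanced Input movement, a dodge roll, health, stamina, stuns and interaction, plus HUD creation.
; Tick regenerates stamina, times out stuns and drives the roll along the last input or mesh facing.
; Rolls cost stamina, have a cooldown, are blocked by stun and negate health damage.
; Body overlaps open a gate for interact input; death only prints and refills health.
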(event OnComponentBeginOverlap(Body)
  (params (OverlappedComponent :type Primitive%20Component%20Object%20Reference) (OtherActor :type Actor%20Object%20Reference) (OtherComp :type Primitive%20Component%20Object%20Reference) (OtherBodyIndex :type Integer) (bFromSweep :type Boolean) (SweepResult :type Hit%20Result%20Structure%20%28by%20ref%29))
  ;[0.15 0.15 0.15 0.5] Interactables
  (bind _asbpi_is_interactable (Utilities|Casting|CastToBPI_IsInteractable OtherActor))
  (Utilities|FlowControl|Gate true) ; enters at Open
)

(event OnComponentEndOverlap(Body)
  (params (OverlappedComponent :type Primitive%20Component%20Object%20Reference) (OtherActor :type Actor%20Object%20Reference) (OtherComp :type Primitive%20Component%20Object%20Reference) (OtherBodyIndex :type Integer))
  ;[0.15 0.15 0.15 0.5] Interactables
  (Utilities|Casting|CastToBPI_IsInteractable OtherActor)
  (Utilities|FlowControl|Gate true) ; enters at Close
)

(event Custom|DestoryComponent_Event
  (params (NewParam :type Actor%20Component%20Object%20Reference))
  ;[0.15 0.15 0.15 0.5] Destroy hitbox
  (Components|DestroyComponent NewParam))

(event Input|EnhancedActionEvents|EnhancedInputActionIA_Roll
  (params (ActionValue :type Boolean) (ElapsedSeconds :type Float%20%28double-precision%29) (TriggeredSeconds :type Float%20%28double-precision%29) (InputAction :type Input%20Action%20Object%20Reference :default "/Game/Blueprints/Input/IA_Roll.IA_Roll"))
  ;[0.15 0.15 0.15 0.5] Toggle Roll
  (if (not (Variables|Default|GetIsRolling))
    (if (not (Variables|Default|GetIsStunned))
      (if (>= (- (Utilities|Time|GetTimeSeconds) (Variables|Default|GetRollCooldownStartTime)) (Variables|Default|GetRoolCooldown))
        (bind _costenough (CallFunction|UseStamina (Variables|Default|GetRollStaminaCost)))
        (if _costenough
          (Variables|Default|SetIsRolling true)
          (Variables|Default|SetRollStartTime (Utilities|Time|GetTimeSeconds))
          (Variables|/Script/Engine.CharacterMovementComponent|SetMaxWalkSpeed (Variables|Character|GetCharacterMovement) (Variables|Default|GetRollSpeed)))))))

(event Input|EnhancedActionEvents|EnhancedInputActionIA_Move
  (params (ActionValue :type Vector%202D%20Structure) (ElapsedSeconds :type Float%20%28double-precision%29) (TriggeredSeconds :type Float%20%28double-precision%29) (InputAction :type Input%20Action%20Object%20Reference :default "/Game/Blueprints/Input/IA_Move.IA_Move"))
  (bind _camera (Variables|Default|GetCamera))
  (bind _camera_2 (Variables|Default|GetCamera))
  (bind _returnvalue (Transformation|GetWorldRotation _camera_2))
  (bind _returnvalue_2 (Transformation|GetWorldRotation _camera))
  (bind _returnvalue_3 (Math|Vector|GetRightVector (Math|Rotator|MakeRotator 0.0 0.0 (.yaw _returnvalue))))
  (bind _returnvalue_4 (Math|Vector|GetForwardVector (Math|Rotator|MakeRotator 0.0 0.0 (.yaw _returnvalue_2))))
  ;[0.15 0.15 0.15 0.5] Player Movement
  (:Triggered
    (if (not (Variables|Default|GetIsRolling))
      (Pawn|Input|AddMovementInput _returnvalue_3 (.x ActionValue) false)
      (Pawn|Input|AddMovementInput _returnvalue_4 (.y ActionValue) false)
      (Variables|Default|SetMovementDirection (+ (* _returnvalue_3 (.x ActionValue)) (* _returnvalue_4 (.y ActionValue))))))
  (:Completed
    ;;[0.15 0.15 0.15 0.5] Reset direction for static rolling
    (Variables|Default|SetMovementDirection "0, 0, 0")))

(event Input|EnhancedActionEvents|EnhancedInputActionIA_Interact
  (params (ActionValue :type Boolean) (ElapsedSeconds :type Float%20%28double-precision%29) (TriggeredSeconds :type Float%20%28double-precision%29) (InputAction :type Input%20Action%20Object%20Reference :default "/Game/Blueprints/Input/IA_Interact.IA_Interact"))
  ;[0.15 0.15 0.15 0.5] Interactables
  (Utilities|FlowControl|Gate true
    (:Exit
      (Default|Interact (stale OnComponentBeginOverlap(Body) _asbpi_is_interactable)))))

(event EventTick
  (params (DeltaSeconds :type Float%20%28single-precision%29))
  (bind _charactermovement (Variables|Character|GetCharacterMovement))
  (bind _stamina (Variables|Default|GetStamina))
  (Utilities|FlowControl|Sequence
    (:then_0
      ;[0.15 0.15 0.15 0.5] Stamina Regen
      (if (>= (- (Utilities|Time|GetTimeSeconds) (Variables|Default|GetStaminaRegenLastTime)) (Variables|Default|GetStaminRegenRate))
        (if (< _stamina (Variables|Default|GetStaminaMax))
          (CallFunction|RegenStamina)
          (Variables|Default|SetStaminaRegenLastTime (Utilities|Time|GetTimeSeconds))
          (Development|PrintString (Utilities|String|ToString(Float) _stamina)))))
    (:then_1
      ;[0.15 0.15 0.15 0.5] Check if Player is Rolling
      (if (Variables|Default|GetIsRolling)
        ;[0.15 0.15 0.15 0.5] End Roll if duration is met or exceeded
        (if (>= (- (Utilities|Time|GetTimeSeconds) (Variables|Default|GetRollStartTime)) (Variables|Default|GetRollDurationSeconds))
          (Variables|Default|SetIsRolling false)
          (Variables|Default|SetRollCooldownStartTime (Utilities|Time|GetTimeSeconds))
          (Variables|/Script/Engine.CharacterMovementComponent|SetMaxWalkSpeed (Variables|Character|GetCharacterMovement) (Variables|Default|GetMaxMoveSpeed))
          (else
            ;[0.15 0.15 0.15 0.5] Roll while rolling state is active (if input direction is empty (0) we just go in the player's view direction)
            (if (Utilities|Operators|EqualEqual :A (Variables|Default|GetMovementDirection))
              (Class|PawnMovementComponent|AddInputVector _charactermovement (Math|Vector|GetForwardVector (Transformation|GetWorldRotation (Variables|Character|GetMesh))) false)
              (else
                (Class|PawnMovementComponent|AddInputVector _charactermovement (Variables|Default|GetMovementDirection) false)))))))
    (:then_2
      ;[0.15 0.15 0.15 0.5] Stun Duration
      (if (>= (- (Utilities|Time|GetTimeSeconds) (Variables|Default|GetStunStartTime)) (Variables|Default|GetStunDurationSeconds))
        (Variables|Default|SetIsStunned false)))))

(event EventBeginPlay
  ;[0.15 0.15 0.15 0.5] Add mapping context for inputs
  (bind _asbp_player_controller (Utilities|Casting|CastToBP_PlayerController (Pawn|GetController)))
  (Utilities|IsValid (PlayerController|LocalPlayerSubsystems|GetEnhancedInputLocalPlayerSubsystem _asbp_player_controller)
    (:Is%20Valid
      (Input|AddMappingContext (PlayerController|LocalPlayerSubsystems|GetEnhancedInputLocalPlayerSubsystem _asbp_player_controller) "/Game/Blueprints/Input/IMC_PlayerMovement.IMC_PlayerMovement" 0 "(bIgnoreAllPressedKeysUntilRelease=True,bForceImmediately=False,bNotifyUserSettings=False)")
      ;[0.15 0.15 0.15 0.5] Destroy hitbox
      (EventDispatchers|BindEventtoDestoryComponent (delegate Custom|DestoryComponent_Event))
      ;[0.15 0.15 0.15 0.5] Initialise Player
      (Variables|Default|SetStamina (Variables|Default|GetStaminaMax))
      (Variables|Default|SetHealth (Variables|Default|GetHealthMax))
      (bind _returnvalue (UserInterface|CreateWidget "/Game/Blueprints/Widgets/InGameHud.InGameHud_C"))
      (bind _output_get (Variables|Default|SetHUDRef _returnvalue))
      (UserInterface|Viewport|AddtoViewport _output_get 0))))

(event Game|Damage|EventAnyDamage
  (params (Damage :type Float%20%28single-precision%29) (DamageType :type Damage%20Type%20Object%20Reference) (InstigatedBy :type Controller%20Object%20Reference) (DamageCauser :type Actor%20Object%20Reference))
  ;[0.15 0.15 0.15 0.5] Take damage so long as the inflictor isn't the player themself
  (if (not (== DamageCauser self))
    (if (Variables|Default|GetIsStunned)
      _
      (else
        (Utilities|Casting|CastToStunDamageType DamageType
          (:then
            (Variables|Default|SetIsStunned true)
            (Variables|Default|SetStunStartTime (Utilities|Time|GetTimeSeconds)))
          (:CastFailed
            _))))
    (CallFunction|TakeDamage Damage)))

(fn ConstructionScript)

(fn TakeDamage
  (params (Damage :type Float%20%28double-precision%29))
  (if (not (Variables|Default|GetIsRolling))
    (bind _output_get (Variables|Default|SetHealth (- (Variables|Default|GetHealth) Damage)))
    (if (<= _output_get 0.0)
      (CallFunction|KIllPlayer))))

(fn KIllPlayer
  (Development|PrintString "Player Died")
  (Variables|Default|SetHealth (Variables|Default|GetHealthMax)))

(fn HealPlayer
  (params (Healing :type Float%20%28double-precision%29))
  (bind _output_get (Variables|Default|SetHealth (Math|Float|Clamp(Float) (+ Healing (Variables|Default|GetHealth)) 0.0 (Variables|Default|GetHealthMax))))
  (Development|PrintString (Utilities|String|ToString(Float) _output_get))
  (Development|PrintString "Player Healed"))

(fn RegenStamina
  (bind _staminamax (Variables|Default|GetStaminaMax))
  (if (> (+ (Variables|Default|GetStamina) (Variables|Default|GetStaminaRegenAmount)) _staminamax)
    (Variables|Default|SetStamina _staminamax)
    (else
      (Variables|Default|SetStamina (+ (Variables|Default|GetStamina) (Variables|Default|GetStaminaRegenAmount))))))

(fn UseStamina
  (params (StaminaCost :type Float%20%28double-precision%29))
  (if (>= (Variables|Default|GetStamina) (Variables|Default|GetRollStaminaCost))
    (Variables|Default|SetStamina (- (Variables|Default|GetStamina) (Variables|Default|GetRollStaminaCost)))
    (return true)
    (else
      (return false))))