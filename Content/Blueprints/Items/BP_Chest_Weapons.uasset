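; Weapon chest that the player can open once to release a random item from its Items list.
; An overlap range toggles the prompt widget, and Interact plays a timeline that rotates the lid hinge.
; When the timeline finishes, the item spawns and Tick accelerates it along a spline.
; At the spline's end, optional landing particles spawn every tick, as Spawned is never cleared.
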(event OnComponentBeginOverlap(InteractionRange)
  (params (OverlappedComponent :type Primitive%20Component%20Object%20Reference) (OtherActor :type Actor%20Object%20Reference) (OtherComp :type Primitive%20Component%20Object%20Reference) (OtherBodyIndex :type Integer) (bFromSweep :type Boolean) (SweepResult :type Hit%20Result%20Structure%20%28by%20ref%29))
  ;[0.15 0.15 0.15 0.5] Show Widget if player is in range and not opened
  (if (not (Variables|Logic|GetOpened))
    (if (== OtherActor (Game|GetPlayerCharacter 0))
      (Rendering|SetVisibility (Variables|Default|GetWidget) true false))))

(event OnComponentEndOverlap(InteractionRange)
  (params (OverlappedComponent :type Primitive%20Component%20Object%20Reference) (OtherActor :type Actor%20Object%20Reference) (OtherComp :type Primitive%20Component%20Object%20Reference) (OtherBodyIndex :type Integer))
  (bind _returnvalue (Game|GetPlayerCharacter 0))
  ;[0.15 0.15 0.15 0.5] Hide widget if player exits and is no longer in range
  (if (== _returnvalue OtherActor)
    ;;[0.15 0.15 0.15 0.5] Check Overlapping actors for the player
    (for _array_element (Collision|GetOverlappingActors (Variables|Default|GetInteraction%20Range) 0 :!class /Script/Engine.PrimitiveComponent)
      ;;[0.15 0.15 0.15 0.5] Stop it from hiding if player is still there
      (if (not (!= _returnvalue _array_element))
        (Variables|Logic|SetPlayer%20In%20range true)))
    (if (Variables|Logic|GetPlayer%20In%20range)
      _
      (else
        (Rendering|SetVisibility (Variables|Default|GetWidget) false false)))
    (Variables|Logic|SetPlayer%20In%20range false)))

(event Custom|Spawn
  (bind _returnvalue (Transformation|GetActorTransform))
  (bind (_location _rotation) (Math|Transform|BreakTransform _returnvalue))
  ;[0.15 0.15 0.15 0.5] Spawn Items
  (bind _returnvalue_2 (Game|SpawnActorfromClass (.OutItem (Utilities|Array|Random (Variables|Spawnable|GetItems))) (Math|Transform|MakeTransform _location (Math|Rotator|MakeRotator 0.0 0.0 (.yaw _rotation)) "1.000000,1.000000,1.000000") "AlwaysSpawn" "MultiplyWithRoot" 0 0))
  (Variables|Logic|SetSpawned true))

(event Custom|Open
  ;[0.15 0.15 0.15 0.5] Open Lid
  (Variables|Logic|SetOpened true)
  (bind _lid_movement (Timeline|Opening%20lid Play)
    (:Update
      (Transformation|AddLocalRotation (Variables|Default|GetHinge) (Math|Rotator|MakeRotator 0.0 0.0 _lid_movement) false false)
      (CallFunction|HideWidget))
    (:Finished
      (CallFunction|Spawn))))

(event Custom|Hide%20Widget
  ;[0.15 0.15 0.15 0.5] Hide widget if player exits and is no longer in range
  (Rendering|SetVisibility (Variables|Default|GetWidget) false false)
  (Variables|Logic|SetPlayer%20In%20range false))

(event EventBeginPlay)

(event EventInteract
  (params (Player :type BP%20Player%20Character%20Object%20Reference))
  (if (not (Variables|Logic|GetOpened))
    (CallFunction|Open)))

(event EventTick
  (params (DeltaSeconds :type Float%20%28single-precision%29))
  ;[0.15 0.15 0.15 0.5] Spawn Items
  ;;[0.15 0.15 0.15 0.5] Check if spawned
  (if (Variables|Logic|GetSpawned)
    ;;[0.15 0.15 0.15 0.5] Acceleration
    (if (>= (Variables|Stats|GetStart%20Speed) (Variables|Stats|GetMax%20Speed))
      _
      (else
        (Variables|Stats|SetStart%20Speed (+ (* DeltaSeconds (Variables|Stats|GetAcceleration)) (Variables|Stats|GetStart%20Speed)))))
    ;;[0.15 0.15 0.15 0.5] Position along spline
    (bind _output_get (Variables|Logic|SetSpline%20Position (+ (* DeltaSeconds (Variables|Stats|GetStart%20Speed)) (Variables|Logic|GetSpline%20Position))))
    ;;[0.15 0.15 0.15 0.5] Move item along spline
    (Transformation|SetWorldTransform (Variables|/Script/Engine.Actor|GetRootComponent (stale Custom|Spawn _returnvalue_2)) (Math|Transform|MakeTransform (.location (Spline|GetTransformatDistanceAlongSpline (Variables|Default|GetSpline) _output_get "World" false)) (Math|Rotator|MakeRotator 0.0 0.0 (.yaw (.Rotation (Math|Transform|BreakTransform (Transformation|GetActorTransform))))) "1.000000,1.000000,1.000000") false false)
    ;;[0.15 0.15 0.15 0.5] Has the end been reached
    (if (>= (Variables|Logic|GetSpline%20Position) (Spline|GetSplineLength (Variables|Default|GetSpline)))
      ;;[0.15 0.15 0.15 0.5] Possible particles
      (if (Variables|Stats|GetSpawn%20Landing%20Particles)
        (bind _returnvalue (Game|SpawnActorfromClass (Variables|Spawnable|GetLanding%20Particles) (Math|Transform|MakeTransform (Transformation|GetWorldLocation (Variables|/Script/Engine.Actor|GetRootComponent (stale Custom|Spawn _returnvalue_2))) "0, 0, 0" "1.000000,1.000000,1.000000") "Undefined" "MultiplyWithRoot" 0 0))
        (Actor|SetLifeSpan _returnvalue (Variables|Stats|GetParticle%20Lifestpan))))))

(fn ConstructionScript
  (bind _interaction_range_ (Variables|Stats|GetInteraction%20Range%20))
  (Transformation|SetWorldScale3D (Variables|Default|GetInteraction%20Range) (Math|Vector|MakeVector _interaction_range_ _interaction_range_ _interaction_range_)))