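; Combat controller component for the player controller that routes combat input to active item components and processes their hitboxes.
; On BeginPlay it adds the combat mapping context and binds component add/remove events that maintain the active item set.
; M1/M2 inputs message the first item through an event switch, which also supports three specials.
; Items register hitboxes, which are evaluated every Tick, with overlap results messaged back to the calling component.
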(event Custom|CallComponentEvent
  (params (Event :type String) (Component :type Actor%20Component%20Object%20Reference))
  (bind _self self)
  ;[0.15 0.15 0.15 0.5] Event switch
  (switch string Event
    (:Default
      (Development|PrintString "Default" true true "(R=1.000000,G=0.000000,B=0.000000,A=1.000000)"))
    (:M1
      (Class|BPICombatInterface|M1(Message) Component _self))
    (:M2
      (Class|BPICombatInterface|M2(Message) Component _self))
    (:Special1
      (Class|BPICombatInterface|Special1(Message) Component _self))
    (:Special2
      (Class|BPICombatInterface|Special2(Message) Component _self))
    (:Special3
      (Class|BPICombatInterface|Special3(Message) Component _self))))

(event Custom|OnComponentAddedComponent_Event
  (params (BlueprintComponent :type Actor%20Component%20Object%20Reference))
  ;[0.15 0.15 0.15 0.5] sets up inputs and bindings
  (Utilities|Set|Add (Variables|Default|GetCurrentActiveItems) BlueprintComponent)
  (Development|PrintString (Utilities|GetDisplayName BlueprintComponent)))

(event Custom|OnComponentRemovedComponent_Event
  (params (Blueprint%20Component :type Actor%20Component%20Object%20Reference))
  ;[0.15 0.15 0.15 0.5] sets up inputs and bindings
  (Utilities|Set|Remove (Variables|Default|GetCurrentActiveItems) Blueprint%20Component)
  (Development|PrintString (Utilities|GetDisplayName Blueprint%20Component)))

(event Input|EnhancedActionEvents|EnhancedInputActionIA_M1
  (params (ActionValue :type Boolean) (ElapsedSeconds :type Float%20%28double-precision%29) (TriggeredSeconds :type Float%20%28double-precision%29) (InputAction :type Input%20Action%20Object%20Reference :default "/Game/Blueprints/Combat/Inputs/InputActions/IA_M1.IA_M1"))
  ;[0.15 0.15 0.15 0.5] Inputs
  (CallFunction|CallComponentEvent "M1" (Utilities|Set|GetItemByIndex (Variables|Default|GetCurrentActiveItems))))

(event Input|EnhancedActionEvents|EnhancedInputActionIA_M2
  (params (ActionValue :type Boolean) (ElapsedSeconds :type Float%20%28double-precision%29) (TriggeredSeconds :type Float%20%28double-precision%29) (InputAction :type Input%20Action%20Object%20Reference :default "/Game/Blueprints/Combat/Inputs/InputActions/IA_M2.IA_M2"))
  ;[0.15 0.15 0.15 0.5] Inputs
  (CallFunction|CallComponentEvent "M2" (Utilities|Set|GetItemByIndex (Variables|Default|GetCurrentActiveItems))))

(event EventBeginPlay
  ;[0.15 0.15 0.15 0.5] sets up inputs and bindings
  (bind _asbp_player_controller (Utilities|Casting|CastToBP_PlayerController (Components|GetOwner)))
  (Variables|Default|SetPlayerController _asbp_player_controller)
  (Input|AddMappingContext (PlayerController|LocalPlayerSubsystems|GetEnhancedInputLocalPlayerSubsystem _asbp_player_controller) "/Game/Blueprints/Combat/Inputs/IMC_Combat.IMC_Combat" 0 "(bIgnoreAllPressedKeysUntilRelease=True,bForceImmediately=False,bNotifyUserSettings=False)")
  (EventDispatchers|BindEventtoOnComponentAddedComponent (delegate Custom|OnComponentAddedComponent_Event))
  (EventDispatchers|BindEventtoOnComponentRemovedComponent (delegate Custom|OnComponentRemovedComponent_Event)))

(event EventTick
  (params (DeltaSeconds :type Float%20%28single-precision%29))
  (bind (_callingcomponent _return_value _hit _hitbox_data) (CallFunction|HitboxTick2 (Variables|Default|GetHitboxes)))
  (Class|BPICombatInterface|OnHitboxOverlap(Message) _callingcomponent _return_value _hit _hitbox_data))

(event EventAddHitboxtoCombatController
  (params (Hitbox :type Struct%20Hitbox%20Data%20Structure) (CallingComponent :type Actor%20Component%20Object%20Reference))
  (CallFunction|Createhitbox (Variables|Default|GetHitboxes) Hitbox CallingComponent))