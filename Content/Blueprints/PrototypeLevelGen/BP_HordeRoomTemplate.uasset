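; BP_HordeRoomTemplate is a prototype level-generation room template with exit logic for moving the player to the next level.
; Four direction branches use TransformPlayerPos to store a target's world location and rotation, though only East supplies a target.
; They share a LevelBeaten check that passes the spawn transform to LoadNextLevel on BP_MainGameInstance.
; No event triggers these branches, so none currently run.
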(fn ConstructionScript)

(fn TransformPlayerPos
  (params (Target :type Capsule%20Component%20Object%20Reference))
  (Variables|Default|SetPlayerSpawnVector (Transformation|GetWorldLocation Target))
  (Variables|Default|SetPlayerSpawnRot (Transformation|GetWorldRotation Target))
  (return))