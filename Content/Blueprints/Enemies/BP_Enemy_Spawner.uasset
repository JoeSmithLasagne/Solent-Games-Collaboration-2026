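; Enemy spawner that emits counted mythical enemies on BeginPlay or Trigger, destroying itself when empty unless it is a non-final wave.
; Type events decrement counts, spawn AI within a square around the actor via SpawnUniversal, then loop after a fixed or random delay.
; Selection follows fixed order or RandomSpawnChooser, which ignores its random roll and picks the last available type.
; The overlap check's result is unused, so it never affects placement.
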(event Custom|Hydra%20Spawn
  ;[0.15 0 0.1126] Hydra
  (Math|Integer|DecrementInt (Variables|EnemiestoSpawn|GetHydra)
    (:%20%20
      (CallFunction|SpawnUniversal (Variables|EnemiesDefinitions|GetHydra%20definition) (Variables|EnemiesBehaviours|GetHydra%20Behavior))
      (CallFunction|Return))))

(event Custom|Chimera%20Spawn
  ;[0.15 0.08422 0 1] Chimera
  (Math|Integer|DecrementInt (Variables|EnemiestoSpawn|GetChimera)
    (:%20%20
      (CallFunction|SpawnUniversal (Variables|EnemiesDefinitions|GetChimera%20definition) (Variables|EnemiesBehaviours|GetChimera%20Behavior))
      (CallFunction|Return))))

(event Custom|Posessed%20Armour%20Spawn
  ;[0.2323 0.2323 0.2323] Posessed Armour
  (Math|Integer|DecrementInt (Variables|EnemiestoSpawn|GetPosessed%20Armour)
    (:%20%20
      (CallFunction|SpawnUniversal (Variables|EnemiesDefinitions|GetPosessed%20Armour%20definition) (Variables|EnemiesBehaviours|GetPossesed%20Armour%20Behavior))
      (CallFunction|Return))))

(event Custom|Harpy%20Spawn
  ;[0.04719 0.1963 0.374] Harpy
  (Math|Integer|DecrementInt (Variables|EnemiestoSpawn|GetHarpy)
    (:%20%20
      (CallFunction|SpawnUniversal (Variables|EnemiesDefinitions|GetHarpy%20definition) (Variables|EnemiesBehaviours|GetHarpy%20Behavior))
      (CallFunction|Return))))

(event Custom|Return
  ;[0.15 0.15 0.15 0.5] Return from an execution
  (Utilities|SpawnDelay
    (:Completed
      ;[0.15 0.15 0.15 0.5] Random delay
      (if (Variables|SpawnLogic|GetRandom%20Delay)
        (Variables|SpawnLogic|SetDelay%20between%20each%20spawn (Math|Random|RandomFloatinRange (Variables|SpawnLogic|GetDelay%20min) (Variables|SpawnLogic|GetDelay%20max))))
      ;[0.15 0.15 0.15 0.5] Random spawn order
      (if (Variables|SpawnLogic|GetRandom%20spawn%20order)
        (bind _done (CallFunction|CheckifDoneSpawning))
        (if _done
          (CallFunction|EndOfLifeHandling)
          (else
            (CallFunction|RandomSpawnChooser)))
        (else
          (CallFunction|DefaultSpawnSelection))))))

(event Custom|Gnome%20Spawn
  ;[0 0.2716 0.2865] Gnome
  (Math|Integer|DecrementInt (Variables|EnemiestoSpawn|GetGnome)
    (:%20%20
      (CallFunction|SpawnUniversal (Variables|EnemiesDefinitions|GetGnome%20definition) (Variables|EnemiesBehaviours|GetGnome%20Behavior))
      (CallFunction|Return))))

(event Custom|Trigger
  ;[0.15 0.15 0.15 0.5] Trigger form game instance
  (if (Variables|SpawnLogic|GetTriggerable%20spawn)
    ;[0.15 0.15 0.15 0.5] Random delay
    (if (Variables|SpawnLogic|GetRandom%20Delay)
      (Variables|SpawnLogic|SetDelay%20between%20each%20spawn (Math|Random|RandomFloatinRange (Variables|SpawnLogic|GetDelay%20min) (Variables|SpawnLogic|GetDelay%20max))))
    ;[0.15 0.15 0.15 0.5] Random spawn order
    (if (Variables|SpawnLogic|GetRandom%20spawn%20order)
      (bind _done (CallFunction|CheckifDoneSpawning))
      (if _done
        (CallFunction|EndOfLifeHandling)
        (else
          (CallFunction|RandomSpawnChooser)))
      (else
        (CallFunction|DefaultSpawnSelection)))))

(event Custom|Basilisk%20Spawn
  ;[0.01096 0.07396 0] Basilisk
  (Math|Integer|DecrementInt (Variables|EnemiestoSpawn|GetBasilisk)
    (:%20%20
      (CallFunction|SpawnUniversal (Variables|EnemiesDefinitions|GetBasilisk%20definition) (Variables|EnemiesBehaviours|GetBasilisk%20Behavior))
      (CallFunction|Return))))

(event Custom|Skeleton%20Spawn
  ;[1 1 1] Skeleton With Shield
  (Math|Integer|DecrementInt (Variables|EnemiesToSpawn|GetSkeleton%20with%20a%20shield)
    (:%20%20
      (CallFunction|SpawnUniversal (Variables|EnemiesDefinitions|GetSkeleton%20definition) (Variables|EnemiesBehaviours|GetSkeleton%20Behavior))
      (CallFunction|Return))))

(event Custom|Shieldless%20Skeleton%20Spawn
  ;[1 1 1] Skeleton Without Shield
  (Math|Integer|DecrementInt (Variables|EnemiesToSpawn|GetSkeleton%20without%20shield)
    (:%20%20
      (bind _newparam (CallFunction|SpawnUniversal (Variables|EnemiesDefinitions|GetSkeleton%20definition) (Variables|EnemiesBehaviours|GetSkeleton%20Behavior)))
      (bind _asbp_skeleton_shield (Utilities|Casting|CastToBP_Skeleton_Shield _newparam))
      (Variables|/Game/Blueprints/Enemies/Skeletons/BP_Skeleton_Shield.BP_Skeleton_Shield_C|SetHits%20To%20Break%20Shield _asbp_skeleton_shield 0)
      (CallFunction|Return))))

(event Custom|Spider%20Spawn
  ;[0 0 0] Spider
  (Math|Integer|DecrementInt (Variables|EnemiestoSpawn|GetSpider)
    (:%20%20
      (CallFunction|SpawnUniversal (Variables|EnemiesDefinitions|GetSpider%20definition) (Variables|EnemiesBehaviours|GetSpider%20Behavior))
      (CallFunction|Return))))

(event EventBeginPlay
  ;[0.15 0.15 0.15 0.5] How to spawn
  (if (not (Variables|SpawnLogic|GetTriggerable%20spawn))
    ;[0.15 0.15 0.15 0.5] User error negation
    (if (Variables|SpawnLogic|GetWaves)
      (Variables|SpawnLogic|SetTriggerable%20spawn true))
    ;[0.15 0.15 0.15 0.5] First spawn delay
    (Utilities|FlowControl|Delay (Variables|SpawnLogic|GetDelay%20for%20first%20enemy))
    ;[0.15 0.15 0.15 0.5] Random delay
    (if (Variables|SpawnLogic|GetRandom%20Delay)
      (Variables|SpawnLogic|SetDelay%20between%20each%20spawn (Math|Random|RandomFloatinRange (Variables|SpawnLogic|GetDelay%20min) (Variables|SpawnLogic|GetDelay%20max))))
    ;[0.15 0.15 0.15 0.5] Random spawn order
    (if (Variables|SpawnLogic|GetRandom%20spawn%20order)
      (bind _done (CallFunction|CheckifDoneSpawning))
      (if _done
        (CallFunction|EndOfLifeHandling)
        (else
          (CallFunction|RandomSpawnChooser)))
      (else
        (CallFunction|DefaultSpawnSelection)))))

(fn ConstructionScript
  (Transformation|SetWorldScale3D (Variables|Default|GetSpawn%20Radius%20Sphere) (Math|Conversions|ToVector(Float) (Variables|SpawnLogic|GetSpawn%20Radius))))

(fn RandomSpawnChooser
  (Variables|InternalLogic|SetAmount%20of%20choices 0)
  (if (> (Variables|EnemiesToSpawn|GetSkeleton%20with%20a%20shield) 0)
    (Math|Integer|IncrementInt (Variables|InternalLogic|GetAmount%20of%20choices)
      (:%20%20
        _)))
  (if (> (Variables|EnemiesToSpawn|GetSkeleton%20without%20shield) 0)
    (Math|Integer|IncrementInt (Variables|InternalLogic|GetAmount%20of%20choices)
      (:%20%20
        _)))
  (if (> (Variables|EnemiestoSpawn|GetSpider) 0)
    (Math|Integer|IncrementInt (Variables|InternalLogic|GetAmount%20of%20choices)
      (:%20%20
        _)))
  (if (> (Variables|EnemiestoSpawn|GetPosessed%20Armour) 0)
    (Math|Integer|IncrementInt (Variables|InternalLogic|GetAmount%20of%20choices)
      (:%20%20
        _)))
  (if (> (Variables|EnemiestoSpawn|GetGnome) 0)
    (Math|Integer|IncrementInt (Variables|InternalLogic|GetAmount%20of%20choices)
      (:%20%20
        _)))
  (if (> (Variables|EnemiestoSpawn|GetBasilisk) 0)
    (Math|Integer|IncrementInt (Variables|InternalLogic|GetAmount%20of%20choices)
      (:%20%20
        _)))
  (if (> (Variables|EnemiestoSpawn|GetChimera) 0)
    (Math|Integer|IncrementInt (Variables|InternalLogic|GetAmount%20of%20choices)
      (:%20%20
        _)))
  (if (> (Variables|EnemiestoSpawn|GetHarpy) 0)
    (Math|Integer|IncrementInt (Variables|InternalLogic|GetAmount%20of%20choices)
      (:%20%20
        _)))
  (if (> (Variables|EnemiestoSpawn|GetHydra) 0)
    (Math|Integer|IncrementInt (Variables|InternalLogic|GetAmount%20of%20choices)
      (:%20%20
        _)))
  (Variables|InternalLogic|SetCurrent%20Choice 1)
  (Variables|InternalLogic|SetRandom%20choice (Math|Random|RandomIntegerinRange 1 (Variables|InternalLogic|GetAmount%20of%20choices)))
  (Utilities|IsGreaterThan0 (Variables|EnemiesToSpawn|GetSkeleton%20with%20a%20shield)
    (:True
      (Utilities|CheckRandomSpawn
        (:Spawn
          (CallFunction|SkeletonSpawn))
        (:Continue
          (Utilities|IsGreaterThan0 (Variables|EnemiesToSpawn|GetSkeleton%20without%20shield) :!label _label
            (:True
              (Utilities|CheckRandomSpawn
                (:Spawn
                  (CallFunction|ShieldlessSkeletonSpawn))
                (:Continue
                  (Utilities|IsGreaterThan0 (Variables|EnemiestoSpawn|GetSpider) :!label _label_2
                    (:True
                      (Utilities|CheckRandomSpawn
                        (:Spawn
                          (CallFunction|SpiderSpawn))
                        (:Continue
                          (Utilities|IsGreaterThan0 (Variables|EnemiestoSpawn|GetPosessed%20Armour) :!label _label_3
                            (:True
                              (Utilities|CheckRandomSpawn
                                (:Spawn
                                  (CallFunction|PosessedArmourSpawn))
                                (:Continue
                                  (Utilities|IsGreaterThan0 (Variables|EnemiestoSpawn|GetGnome) :!label _label_4
                                    (:True
                                      (Utilities|CheckRandomSpawn
                                        (:Spawn
                                          (CallFunction|GnomeSpawn))
                                        (:Continue
                                          (Utilities|IsGreaterThan0 (Variables|EnemiestoSpawn|GetBasilisk) :!label _label_5
                                            (:True
                                              (Utilities|CheckRandomSpawn
                                                (:Spawn
                                                  (CallFunction|BasiliskSpawn))
                                                (:Continue
                                                  (Utilities|IsGreaterThan0 (Variables|EnemiestoSpawn|GetChimera) :!label _label_6
                                                    (:True
                                                      (Utilities|CheckRandomSpawn
                                                        (:Spawn
                                                          (CallFunction|ChimeraSpawn))
                                                        (:Continue
                                                          (Utilities|IsGreaterThan0 (Variables|EnemiestoSpawn|GetHarpy) :!label _label_7
                                                            (:True
                                                              (Utilities|CheckRandomSpawn
                                                                (:Spawn
                                                                  (CallFunction|HarpySpawn))
                                                                (:Continue
                                                                  (Utilities|IsGreaterThan0 (Variables|EnemiestoSpawn|GetHydra) :!label _label_8
                                                                    (:True
                                                                      (Utilities|CheckRandomSpawn
                                                                        (:Spawn
                                                                          (CallFunction|HydraSpawn))
                                                                        (:Continue
                                                                          ;[0.15 0.15 0.15 0.5] On error
                                                                          (CallFunction|Return :!label _label_9))))
                                                                    (:False
                                                                      (goto _label_9))))))
                                                            (:False
                                                              (goto _label_8))))))
                                                    (:False
                                                      (goto _label_7))))))
                                            (:False
                                              (goto _label_6))))))
                                    (:False
                                      (goto _label_5))))))
                            (:False
                              (goto _label_4))))))
                    (:False
                      (goto _label_3))))))
            (:False
              (goto _label_2))))))
    (:False
      (goto _label))))

(fn CheckifDoneSpawning
  (return (Math|Boolean|ANDBoolean (<= (Variables|EnemiesToSpawn|GetSkeleton%20with%20a%20shield) 0) (<= (Variables|EnemiesToSpawn|GetSkeleton%20without%20shield) 0) (<= (Variables|EnemiestoSpawn|GetSpider) 0) (<= (Variables|EnemiestoSpawn|GetPosessed%20Armour) 0) (<= (Variables|EnemiestoSpawn|GetGnome) 0) (<= (Variables|EnemiestoSpawn|GetBasilisk) 0) (<= (Variables|EnemiestoSpawn|GetChimera) 0) (<= (Variables|EnemiestoSpawn|GetHarpy) 0) (<= (Variables|EnemiestoSpawn|GetHydra) 0))))

(fn RandomSpawnRadiusCalculations
  (bind _returnvalue (Transformation|GetActorTransform))
  (bind _spawn_radius (Variables|SpawnLogic|GetSpawn%20Radius))
  (bind _spawn_radius_2 (Variables|SpawnLogic|GetSpawn%20Radius))
  (bind _returnvalue_2 (* _spawn_radius 25.0))
  (bind _returnvalue_3 (+ (.z (.location _returnvalue)) 0.5))
  (bind _returnvalue_4 (* _spawn_radius_2 25.0))
  (bind _returnvalue_5 (* _returnvalue_2 -1.0))
  (bind _returnvalue_6 (* _returnvalue_4 -1.0))
  (bind _returnvalue_7 (Math|Random|RandomFloatinRange _returnvalue_6 _returnvalue_4))
  (bind _returnvalue_8 (Math|Random|RandomFloatinRange _returnvalue_5 _returnvalue_2))
  (bind _returnvalue_9 (+ (.x (.location _returnvalue)) _returnvalue_7))
  (bind _returnvalue_10 (+ (.y (.location _returnvalue)) _returnvalue_8))
  (bind _blocked_spawn (CallFunction|SpawnableCheck (Math|Vector|MakeVector _returnvalue_9 _returnvalue_10 _returnvalue_3)))
  (if _blocked_spawn
    _
    (else
      _))
  (return _returnvalue_9 _returnvalue_10 _returnvalue_3 (.rotation _returnvalue) (.scale _returnvalue)))

(fn EndOfLifeHandling
  ;[0.15 0.15 0.15 0.5] End of life handling
  (if (Variables|SpawnLogic|GetWaves)
    (if (Variables|InternalLogic|GetLast%20Wave)
      (Actor|DestroyActor :!label _label))
    (else
      (goto _label))))

(fn SpawnUniversal
  (params (Enemy%20type :type Pawn%20Class%20Reference) (Behavior :type Behavior%20Tree%20Object%20Reference))
  (bind (_location_x _location_y _location_z _rotation) (CallFunction|RandomSpawnRadiusCalculations))
  (bind _returnvalue (AI|SpawnAIFromClass Enemy%20type Behavior (Math|Vector|MakeVector _location_x _location_y _location_z) _rotation true 0))
  (return _returnvalue))

(fn OverlapCheck
  (params (Overlapping%20actor :type Array%20of%20Actor%20Object%20References) (Radius :type Float%20%28double-precision%29) (Spawn%20Location :type Vector))
  (for _array_element Overlapping%20actor
    (return (Math|Boolean|ORBoolean (>= (.x (- (Transformation|GetActorLocation _array_element) Radius)) (.x Spawn%20Location)) (>= (.z (- (Transformation|GetActorLocation _array_element) Radius)) (.z Spawn%20Location)) (<= (.x (+ (Transformation|GetActorLocation _array_element) Radius)) (.x Spawn%20Location)) (<= (.z (+ (Transformation|GetActorLocation _array_element) Radius)) (.z Spawn%20Location))))))

(fn SpawnableCheck
  (params (Spawn%20Location :type Vector))
  (bind _spawn_radius_sphere (Variables|Default|GetSpawn%20Radius%20Sphere))
  (bind _overlap (CallFunction|OverlapCheck (Collision|GetOverlappingActors _spawn_radius_sphere (Variables|EnemiesDefinitions|GetSkeleton%20definition) :!class /Script/Engine.PrimitiveComponent) (Variables|EnemiesRadius|GetSkeleton%20Radius) Spawn%20Location))
  (bind _overlap_2 (CallFunction|OverlapCheck (Collision|GetOverlappingActors _spawn_radius_sphere (Variables|EnemiesDefinitions|GetSpider%20definition) :!class /Script/Engine.PrimitiveComponent) (Variables|EnemiesRadius|GetSpider%20Radius) Spawn%20Location))
  (bind _overlap_3 (CallFunction|OverlapCheck (Collision|GetOverlappingActors _spawn_radius_sphere (Variables|EnemiesDefinitions|GetPosessed%20Armour%20definition) :!class /Script/Engine.PrimitiveComponent) (Variables|EnemiesRadius|GetPossesed%20Armour%20Radius) Spawn%20Location))
  (bind _overlap_4 (CallFunction|OverlapCheck (Collision|GetOverlappingActors _spawn_radius_sphere (Variables|EnemiesDefinitions|GetGnome%20definition) :!class /Script/Engine.PrimitiveComponent) (Variables|EnemiesRadius|GetGnome%20Radius) Spawn%20Location))
  (bind _overlap_5 (CallFunction|OverlapCheck (Collision|GetOverlappingActors _spawn_radius_sphere (Variables|EnemiesDefinitions|GetBasilisk%20definition) :!class /Script/Engine.PrimitiveComponent) (Variables|EnemiesRadius|GetBasilisk%20Radius) Spawn%20Location))
  (bind _overlap_6 (CallFunction|OverlapCheck (Collision|GetOverlappingActors _spawn_radius_sphere (Variables|EnemiesDefinitions|GetChimera%20definition) :!class /Script/Engine.PrimitiveComponent) (Variables|EnemiesRadius|GetChimera%20Radius) Spawn%20Location))
  (bind _overlap_7 (CallFunction|OverlapCheck (Collision|GetOverlappingActors _spawn_radius_sphere (Variables|EnemiesDefinitions|GetHarpy%20definition) :!class /Script/Engine.PrimitiveComponent) (Variables|EnemiesRadius|GetHarpy%20Radius) Spawn%20Location))
  (bind _overlap_8 (CallFunction|OverlapCheck (Collision|GetOverlappingActors _spawn_radius_sphere (Variables|EnemiesDefinitions|GetHydra%20definition) :!class /Script/Engine.PrimitiveComponent) (Variables|EnemiesRadius|GetHydra%20Radius) Spawn%20Location))
  (return (Math|Boolean|ORBoolean _overlap_8 _overlap_7 _overlap_6 _overlap_5 _overlap_4 _overlap_3 _overlap_2 _overlap)))

(fn DefaultSpawnSelection
  ;[0.15 0.15 0.15 0.5] Default selection progress
  (if (> (Variables|EnemiesToSpawn|GetSkeleton%20with%20a%20shield) 0)
    (CallFunction|SkeletonSpawn)
    (elif (> (Variables|EnemiesToSpawn|GetSkeleton%20without%20shield) 0)
      (CallFunction|ShieldlessSkeletonSpawn)
      (elif (> (Variables|EnemiestoSpawn|GetSpider) 0)
        (CallFunction|SpiderSpawn)
        (elif (> (Variables|EnemiestoSpawn|GetPosessed%20Armour) 0)
          (CallFunction|PosessedArmourSpawn)
          (elif (> (Variables|EnemiestoSpawn|GetGnome) 0)
            (CallFunction|GnomeSpawn)
            (elif (> (Variables|EnemiestoSpawn|GetBasilisk) 0)
              (CallFunction|BasiliskSpawn)
              (elif (> (Variables|EnemiestoSpawn|GetChimera) 0)
                (CallFunction|ChimeraSpawn)
                (elif (> (Variables|EnemiestoSpawn|GetHarpy) 0)
                  (CallFunction|HarpySpawn)
                  (elif (> (Variables|EnemiestoSpawn|GetHydra) 0)
                    (CallFunction|HydraSpawn)
                    (else
                      (CallFunction|EndOfLifeHandling))))))))))))