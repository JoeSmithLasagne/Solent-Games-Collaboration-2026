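; Test combat ability component that registers with the owner's controller on BeginPlay and supplies an M1 attack.
; M1 builds timed hitbox data, offset from the owning actor, and adds it to the combat controller with itself as caller.
; The hitbox overlap callback applies the hitbox's damage, keeping damage handling in the component rather than the controller.
; Component removal logic exists but is not connected.
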(event EventBeginPlay
  (bind _returnvalue (Components|GetOwner))
  (bind _instigator (Variables|/Script/Engine.Actor|GetInstigator _returnvalue))
  (bind _returnvalue_2 (Pawn|GetController _instigator))
  ;[0.15 0.15 0.15 0.5] Adds component to combat controller stack upon being added to character
  (Class|BPICombatInterface|OnComponentAdded(Message) _returnvalue_2 self)
  (Development|PrintString (Utilities|GetDisplayName _returnvalue_2)))

(event EventM1
  (params (CombatController :type Actor%20Component%20Object%20Reference))
  (bind _self self)
  ;[0.15 0.15 0.15 0.5] Create the hitbox data and add it to the combat controller array
  (Class|BPICombatInterface|AddHitboxtoCombatController(Message) CombatController (Utilities|Struct|MakeStruct_HitboxData (Utilities|String|Append (Utilities|GetDisplayName _self) "_M1") (Components|GetOwner _self) true 0.1 (Utilities|Time|GetGameTimeinSeconds) (Utilities|Time|GetWorldDeltaSeconds) 1e+01 (Math|Transform|MakeTransform "125.000000,0.000000,0.000000" "0, 0, 0" "200.000000,100.000000,50.000000") 1.0) _self))

(event EventOnHitboxOverlap
  (params (HasHit? :type Boolean) (Hit :type Hit%20Result%20Structure) (HitboxData :type Struct%20Hitbox%20Inst%20Structure))
  (bind _data (Utilities|Struct|BreakStruct_HitboxInst HitboxData))
  (bind (_key _owning_actor _active _lifetime _starttime _updaterate _damage) (Utilities|Struct|BreakStruct_HitboxData _data))
  ;[0.15 0.15 0.15 0.5] Damage and other effects should be done by the weapon component
  (if HasHit?
    (Game|Damage|ApplyDamage (.HitActor (Collision|BreakHitResult Hit)) _damage (Pawn|GetController (Variables|/Script/Engine.Actor|GetInstigator _owning_actor)) _owning_actor)))