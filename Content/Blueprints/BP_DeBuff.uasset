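; BP_DeBuff is a debug-driven prototype for tracking stacking debuffs in an ActiveDebuff struct array.
; The O key or AddDebuff event picks one of the first two DeBuffDT rows at random, ignoring the passed name.
; Looping over active entries, it increments Count on name matches; each mismatch appends the row and re-calls AddDebuff recursively.
; The P key prints each active debuff's name and count.
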(event Custom|Add%20Debuff
  (params (Debuffname :type Name))
  (bind _activedebuff (Variables|Default|GetActiveDebuff))
  (bind _outrownames (DataTable|GetDataTableRowNames "/Game/Blueprints/Widgets/InGameUi/DeBuffDT.DeBuffDT"))
  (bind _returnvalue (Utilities|GetDataTableRow "/Game/Blueprints/Widgets/InGameUi/DeBuffDT.DeBuffDT" (Utilities|Array|Get(acopy) _outrownames (Math|Random|RandomInteger 2)))
    (:then
      (for _array_element (Variables|Default|GetActiveDebuff)
        (if (== (.name _array_element) (.name _returnvalue))
          (Math|Integer|IncrementInt (.count (Utilities|Array|Get(acopy) _activedebuff (Utilities|Array|FindItem _activedebuff (Utilities|Struct|MakeDeBuffStruct (.name _returnvalue) (.icon _returnvalue) (.debuff _returnvalue) (.buff _returnvalue) (.tooltip _returnvalue) (.type _returnvalue) (.count _returnvalue))))))
          (else
            (Utilities|Array|Add (Variables|Default|GetActiveDebuff) (Utilities|Struct|MakeDeBuffStruct (.name _returnvalue) (.icon _returnvalue) (.debuff _returnvalue) (.buff _returnvalue) (.tooltip _returnvalue) (.type _returnvalue) (.count _returnvalue)))
            (CallFunction|AddDebuff (.name _returnvalue))))))))

(event Input|KeyboardEvents|DebugKeyP
  (params (Key :type Key%20Structure :default "None") (ActionValue :type Input%20Action%20Value%20Structure))
  ;[0.15 0.15 0.15 0.5] Print Debuffs
  (:Pressed
    (for _array_element (Variables|Default|GetActiveDebuff)
      (Development|PrintString (Utilities|String|ToString(Name) (.name _array_element)))
      (Development|PrintString (Utilities|String|ToString(Integer) (.count _array_element))))))

(event Input|KeyboardEvents|DebugKeyO
  (params (Key :type Key%20Structure :default "None") (ActionValue :type Input%20Action%20Value%20Structure))
  (bind _activedebuff (Variables|Default|GetActiveDebuff))
  (:Pressed
    (bind _outrownames (DataTable|GetDataTableRowNames "/Game/Blueprints/Widgets/InGameUi/DeBuffDT.DeBuffDT"))
    (bind _returnvalue (Utilities|GetDataTableRow "/Game/Blueprints/Widgets/InGameUi/DeBuffDT.DeBuffDT" (Utilities|Array|Get(acopy) _outrownames (Math|Random|RandomInteger 2)))
      (:then
        (for _array_element (Variables|Default|GetActiveDebuff)
          (if (== (.name _array_element) (.name _returnvalue))
            (Math|Integer|IncrementInt (.count (Utilities|Array|Get(acopy) _activedebuff (Utilities|Array|FindItem _activedebuff (Utilities|Struct|MakeDeBuffStruct (.name _returnvalue) (.icon _returnvalue) (.debuff _returnvalue) (.buff _returnvalue) (.tooltip _returnvalue) (.type _returnvalue) (.count _returnvalue))))))
            (else
              (Utilities|Array|Add (Variables|Default|GetActiveDebuff) (Utilities|Struct|MakeDeBuffStruct (.name _returnvalue) (.icon _returnvalue) (.debuff _returnvalue) (.buff _returnvalue) (.tooltip _returnvalue) (.type _returnvalue) (.count _returnvalue)))
              (CallFunction|AddDebuff (.name _returnvalue)))))))))