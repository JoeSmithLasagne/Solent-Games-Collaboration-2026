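; Inventory component that holds six typed equipment slots, lets the player pick up nearby items and shows them in a WB_Inventory widget.
; E toggles the widget along with cursor and input mode.
; T sphere-traces around the player for a BP_Item, maps its slot type to a fixed index, then fills that slot or stacks up to 64.
; The widget then reloads and the picked item gets a short lifespan.
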(event EventBeginPlay
  ;[0.15 0.15 0.15 0.5] Creation of the Widget Inventory -- Where the number of slots are decided
  (bind _returnvalue (UserInterface|CreateWidget "/Game/Blueprints/Inventory/Widgets/WB_Inventory.WB_Inventory_C"))
  (Variables|Default|SetInventoryWidget _returnvalue)
  ;;[0.15 0.15 0.15 0.5] Number Slots
  (Utilities|Array|Resize (Variables|Default|GetItems) 6)
  (Default|LoadInventory (Variables|Default|GetInventoryWidget) self)
  (CallFunction|ClasifyItemsIndex "NewEnumerator0"))

(event Input|KeyboardEvents|E
  (params (Key :type Key%20Structure))
  (bind _returnvalue (Game|GetPlayerController 0))
  (bind _returnvalue_2 (Game|GetPlayerController 0))
  (bind _inventorywidget (Variables|Default|GetInventoryWidget))
  ;[0.15 0.15 0.15 0.5] Press E to open the Inventory, character is able to move the mouse ONLY when the Inventory is open
  (:Pressed
    (if (Widget|IsVisible (Variables|Default|GetInventoryWidget))
      ;;[0.15 0.15 0.15 0.5] Mouse NOT showing
      (Variables|/Script/Engine.PlayerController|SetbShowMouseCursor _returnvalue false)
      (Input|SetInputModeGameOnly _returnvalue false)
      (Widget|RemovefromParent _inventorywidget)
      (else
        ;;[0.15 0.15 0.15 0.5] Mouse showing
        (Variables|/Script/Engine.PlayerController|SetbShowMouseCursor _returnvalue_2 true)
        (Input|SetInputModeGameandUI _returnvalue_2 0 "DoNotLock" false false)
        (UserInterface|Viewport|AddtoViewport _inventorywidget 0)))))

(event Input|KeyboardEvents|T
  (params (Key :type Key%20Structure))
  (bind _returnvalue (Game|GetPlayerCharacter 0))
  (bind _returnvalue_2 (Transformation|GetActorLocation _returnvalue))
  (bind _returnvalue_3 (- _returnvalue_2 "0.000000,0.000000,20.000000"))
  ;[0.15 0.15 0.15 0.5] Press T to open the items in the surroundings -- Full process Blueprint
  (:Pressed
    (bind _outhit (Collision|SphereTraceByChannel _returnvalue_3 _returnvalue_3 2e+02 "TraceTypeQuery1" false 0 "None"))
    (bind _asbp_item (Utilities|Casting|CastToBP_Item (.HitActor (Collision|BreakHitResult _outhit)))
      (:then
        (for _array_element (Variables|Default|GetItems)
          (Utilities|IsValid _asbp_item
            (:Is%20Valid
              (bind _index (CallFunction|ClasifyItemsIndex (.SlotType (Utilities|Struct|BreakS_EquipmentSlot (Variables|/Game/Blueprints/Inventory/Blueprints/BP_Item.BP_Item_C|GetItem _asbp_item))) _asbp_item (Variables|Default|GetItems)))
              (if (Math|Boolean|ANDBoolean (Utilities|Enum|Equal(Enum) (.name (.Item (Utilities|Struct|BreakS_EquipmentSlot _array_element))) (.name (.Item (Utilities|Struct|BreakS_EquipmentSlot (Variables|/Game/Blueprints/Inventory/Blueprints/BP_Item.BP_Item_C|GetItem _asbp_item))))) (.stackable (.Item (Utilities|Struct|BreakS_EquipmentSlot (Variables|/Game/Blueprints/Inventory/Blueprints/BP_Item.BP_Item_C|GetItem _asbp_item)))) (<= (+ (.quantity (.Item (Utilities|Struct|BreakS_EquipmentSlot _array_element))) (.quantity (.Item (Utilities|Struct|BreakS_EquipmentSlot (Variables|/Game/Blueprints/Inventory/Blueprints/BP_Item.BP_Item_C|GetItem _asbp_item))))) 64))
                (Utilities|Array|SetArrayElem (Variables|Default|GetItems) _index (Utilities|Struct|MakeS_EquipmentSlot (.SlotType (Utilities|Struct|BreakS_EquipmentSlot (Variables|/Game/Blueprints/Inventory/Blueprints/BP_Item.BP_Item_C|GetItem _asbp_item))) (Utilities|Struct|MakeS_ItemStructure (.name (.Item (Utilities|Struct|BreakS_EquipmentSlot (Variables|/Game/Blueprints/Inventory/Blueprints/BP_Item.BP_Item_C|GetItem _asbp_item)))) (.stackable (.Item (Utilities|Struct|BreakS_EquipmentSlot (Variables|/Game/Blueprints/Inventory/Blueprints/BP_Item.BP_Item_C|GetItem _asbp_item)))) (+ (.quantity (.Item (Utilities|Struct|BreakS_EquipmentSlot _array_element))) (.quantity (.Item (Utilities|Struct|BreakS_EquipmentSlot (Variables|/Game/Blueprints/Inventory/Blueprints/BP_Item.BP_Item_C|GetItem _asbp_item))))) (.thumbnail (.Item (Utilities|Struct|BreakS_EquipmentSlot (Variables|/Game/Blueprints/Inventory/Blueprints/BP_Item.BP_Item_C|GetItem _asbp_item)))) (.mesh (.Item (Utilities|Struct|BreakS_EquipmentSlot (Variables|/Game/Blueprints/Inventory/Blueprints/BP_Item.BP_Item_C|GetItem _asbp_item)))))) true)
                (Default|LoadInventory (Variables|Default|GetInventoryWidget) self :!label _label)
                (Utilities|FlowControl|Sequence
                  (:then_0
                    (Actor|SetLifeSpan _asbp_item 2.0))
                  (:then_1
                    (Components|Activation|Activate (Variables|/Game/Blueprints/Inventory/Blueprints/BP_Item.BP_Item_C|GetSphere _asbp_item) false)))
                (elif (== (.quantity (.Item (Utilities|Struct|BreakS_EquipmentSlot _array_element))) 0)
                  (Utilities|Array|SetArrayElem (Variables|Default|GetItems) _index (Variables|/Game/Blueprints/Inventory/Blueprints/BP_Item.BP_Item_C|GetItem _asbp_item))
                  (goto _label)))))))
      (:CastFailed
        (Development|PrintString "Item not picked!!")))))

(fn ClasifyItemsIndex
  (params (B :type E_SlotType%20Enum :default "NewEnumerator0") (BP_Item :type BP%20Item%20Object%20Reference) (Items :type Array%20of%20S%20Equipment%20Slot%20Structures))
  (Utilities|FlowControl|Sequence
    (:then_0
      (if (== B (Utilities|Enum|LiteralenumE_SlotType "NewEnumerator0"))
        (Variables|Default|SetArray%20Index 0)
        (Utilities|IsValid BP_Item
          (:Is%20Valid
            (bind _output_get (Variables|Default|SetArray%20Index 0))
            (return _output_get)))))
    (:then_1
      (if (Utilities|Enum|Equal(Enum) (Utilities|Enum|LiteralenumE_SlotType "NewEnumerator1") B)
        (Variables|Default|SetArray%20Index 3)
        (Utilities|IsValid BP_Item
          (:Is%20Valid
            (bind _output_get_2 (Variables|Default|SetArray%20Index 3))
            (return _output_get_2)))))
    (:then_2
      (if (Utilities|Enum|Equal(Enum) B (Utilities|Enum|LiteralenumE_SlotType "NewEnumerator2"))
        (Variables|Default|SetArray%20Index 1)
        (Utilities|IsValid BP_Item
          (:Is%20Valid
            (bind _output_get_3 (Variables|Default|SetArray%20Index 1))
            (return _output_get_3)))))
    (:then_3
      (if (Utilities|Enum|Equal(Enum) (Utilities|Enum|LiteralenumE_SlotType "NewEnumerator4") B)
        (Variables|Default|SetArray%20Index 4)
        (Utilities|IsValid BP_Item
          (:Is%20Valid
            (bind _output_get_4 (Variables|Default|SetArray%20Index 4))
            (return _output_get_4)))))
    (:then_4
      (if (Utilities|Enum|Equal(Enum) (Utilities|Enum|LiteralenumE_SlotType "NewEnumerator5") B)
        (Variables|Default|SetArray%20Index 2)
        (Utilities|IsValid BP_Item
          (:Is%20Valid
            (bind _output_get_5 (Variables|Default|SetArray%20Index 2))
            (return _output_get_5)))))
    (:then_5
      (if (Utilities|Enum|Equal(Enum) B (Utilities|Enum|LiteralenumE_SlotType "NewEnumerator6"))
        (Variables|Default|SetArray%20Index 5)
        (Utilities|IsValid BP_Item
          (:Is%20Valid
            (bind _output_get_6 (Variables|Default|SetArray%20Index 5))
            (return _output_get_6)))))))