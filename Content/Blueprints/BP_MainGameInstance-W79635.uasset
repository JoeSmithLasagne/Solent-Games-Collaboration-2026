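; Game instance that drives room-to-room progression, enemy spawning and saved player health stats.
; LoadNextLevel teleports the player, then a DoOnce-guarded step spawns a random room class, destroys the current one and re-enables loading as a placeholder.
; TriggerEnemiesSpawning fires every enemy spawner, handing any pending last-wave flag to the first.
; SaveStats stores health and max health but ignores the move speed input.
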(event Custom|LoadNextLevel
  (params (NewPlayerPos :type Vector) (NewPlayerRot :type Rotator) (CurrentLevel :type Actor%20Object%20Reference))
  (Transformation|SetActorLocationAndRotation (Game|GetPlayerCharacter 0) NewPlayerPos NewPlayerRot false true)
  (Utilities|FlowControl|DoOnce false
    (:Completed
      (Game|SpawnActorfromClass (.OutItem (Utilities|Array|Random (Variables|Default|GetClass))) (Math|Transform|MakeTransform "0, 0, 0" "0, 0, 0" "1.000000,1.000000,1.000000") "Undefined" "MultiplyWithRoot" 0 0)
      (Actor|DestroyActor CurrentLevel)
      ;[0.15 0.15 0.15 0.5] Placeholder until Later
      (CallFunction|AllowLevelLoad))))

(event Custom|AllowLevelLoad
  (bind _outactors (Actor|GetAllActorsOfClass "/Game/Maps/BP_BasicRoomTemplate.BP_BasicRoomTemplate_C"))
  (Default|AllowLevelLoad _outactors)
  (CallFunction|EnableLevelLoad))

(event Custom|EnableLevelLoad
  (Utilities|FlowControl|DoOnce false) ; enters at Reset
)

(fn TriggerEnemiesSpawning
  ;[0.15 0.15 0.15 0.5] Trigger all enemy spawners in the room
  (bind _outactors (Actor|GetAllActorsOfClass "/Game/Blueprints/Enemies/BP_Enemy_Spawner.BP_Enemy_Spawner_C"))
  (for _array_element _outactors
    (Default|Trigger _array_element)
    ;[0.15 0.15 0.15 0.5] Handle the last wave if spawning waves
    (if (Variables|Default|GetLast%20wave)
      (Variables|/Game/Blueprints/Enemies/BP_Enemy_Spawner.BP_Enemy_Spawner_C|SetLast%20Wave _array_element (Variables|Default|GetLast%20wave))
      (Variables|Default|SetLast%20wave false))))

(fn SaveStats
  (params (CurrentHealth :type Float%20%28double-precision%29) (CurrentMaxHealth :type Float%20%28double-precision%29) (CurrentMaxMoveSpeed :type Float%20%28double-precision%29))
  (Variables|Default|SetHealth CurrentHealth)
  (Variables|Default|SetMaxHealth CurrentMaxHealth))