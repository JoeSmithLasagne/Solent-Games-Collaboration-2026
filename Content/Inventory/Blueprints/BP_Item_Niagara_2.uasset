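; BP_Item_Niagara_2 is an inventory item actor that plays a rise-and-vanish animation with Niagara effects.
; The construction script sets its mesh from Item data for editor preview, and BeginPlay deactivates the Sphere.
; The T key activates the Sphere, whose activation event enables input and starts a Timeline that lifts the actor, spawning NiagaraNormal each update before delayed destruction.
; Ending overlap with the Sphere disables input.
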(event OnComponentActivated(Sphere)
  (params (Component :type Actor%20Component%20Object%20Reference) (bReset :type Boolean))
  ;[0.15 0.15 0.15 0.5] Item Animation
  (Input|EnableInput (Game|GetPlayerController 0))
  (Utilities|FlowControl|Delay 0.2)
  (bind _output_get (Variables|Default|SetStartLocation (Transformation|GetActorLocation)))
  (bind _alpha1 (Timeline|Timeline Play)
    (:Update
      (Transformation|SetActorLocation (Math|Vector|Lerp(Vector) _output_get (+ _output_get "0.000000,0.000000,300.000000") _alpha1) false false)
      (Niagara|SpawnSystematLocation "/Game/Blueprints/Animations/NiagaraEffects/NiagaraNormal.NiagaraNormal" (Math|Vector|Lerp(Vector) _output_get (+ _output_get "0.000000,0.000000,300.000000") _alpha1))
      (Utilities|FlowControl|Delay 2.0)
      (Actor|DestroyActor))))

(event OnComponentEndOverlap(Sphere)
  (params (OverlappedComponent :type Primitive%20Component%20Object%20Reference) (OtherActor :type Actor%20Object%20Reference) (OtherComp :type Primitive%20Component%20Object%20Reference) (OtherBodyIndex :type Integer))
  ;[0.15 0.15 0.15 0.5] Item Animation
  (Input|DisableInput 0))

(event EventBeginPlay
  ;[0.15 0.15 0.15 0.5] Object --> Deactivated at the beginning of the Program
  (Components|Activation|Deactivate (Variables|Default|GetSphere)))

(event Collision|EventActorBeginOverlap
  (params (OtherActor :type Actor%20Object%20Reference)))

(event EventTick
  (params (DeltaSeconds :type Float%20%28single-precision%29)))

(event Input|KeyboardEvents|T
  (params (Key :type Key%20Structure :default "None"))
  ;[0.15 0.15 0.15 0.5] Item Animation
  (:Pressed
    (Components|Activation|Activate (Variables|Default|GetSphere) false)))

(fn ConstructionScript
  ;[0.15 0.15 0.15 0.5] Construction Script to see the Item already build before executing the Level
  (Components|StaticMesh|SetStaticMesh (Variables|Default|GetStaticMesh) (.mesh (.Item (Utilities|Struct|BreakS_EquipmentSlot (Variables|Default|GetItem)))))
  (Physics|SetSimulatePhysics (Variables|Default|GetStaticMesh) false))