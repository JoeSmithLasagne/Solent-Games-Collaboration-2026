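; BP_Possessed_Armour is an enemy with health, a healthbar widget, configurable move speed and a debug-stage attack that damages the player.
; Incoming damage passes a DoOnce immunity-frame gate, reset from Tick after a delay.
; Every third hit is ignored, with the hit counter cleared on a looping timer, and ranged damage is also ignored at half health or below.
; Other hits reduce health, update the healthbar and destroy the actor at zero.
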(event Custom|Reset%20Hit%20Counter
  ;[0.15 0.15 0.15 0.5] Reset Hit counter every 4 seconds
  (Variables|Default|SetHit%20Counter 0))

(event Custom|Attack
  ;[0.15 0.15 0.15 0.5] Attack debug
  (Development|PrintString "Attacking")
  ;[0.15 0.15 0.15 0.5] Apply Damage
  (Game|Damage|ApplyDamage (Game|GetPlayerCharacter 0) (Variables|Default|GetAttack_Damage) 0 self))

(event EventTick
  (params (DeltaSeconds :type Float%20%28single-precision%29))
  ;[0.15 0.15 0.15 0.5] Immunity Frames
  (if (Variables|Default|GetHit)
    (Utilities|FlowControl|Delay (Variables|Default|GetImmunity_Frames))
    (Variables|Default|SetHit false)
    (Utilities|FlowControl|DoOnce false) ; enters at Reset
  ))

(event EventBeginPlay
  ;[0.15 0.15 0.15 0.5] Set movement speed
  (Variables|/Script/Engine.CharacterMovementComponent|SetMaxWalkSpeed (Variables|Character|GetCharacterMovement) (Variables|Default|GetMovement_Speed))
  ;[0.15 0.15 0.15 0.5] Set current health
  (Variables|Default|SetCurrent_Health (Variables|Default|GetMax_Health))
  (CallFunction|UpdateHealthbar)
  ;[0.15 0.15 0.15 0.5] Reset Hit counter every 4 seconds
  (Utilities|Time|SetTimerbyEvent (delegate Custom|Reset%20Hit%20Counter) 4.0 true))

(event Game|Damage|EventAnyDamage
  (params (Damage :type Float%20%28single-precision%29) (DamageType :type Damage%20Type%20Object%20Reference) (InstigatedBy :type Controller%20Object%20Reference) (DamageCauser :type Actor%20Object%20Reference))
  ;[0.15 0.15 0.15 0.5] Immunity Frames
  (Utilities|FlowControl|DoOnce false
    (:Completed
      (Variables|Default|SetHit true)
      (if (<= (Variables|Default|GetCurrent_Health) (/ (Variables|Default|GetMax_Health) 2.0))
        (if (not (Utilities|Enum|Equal(Enum) (Variables|Default|GetDamage_Type) "Ranged"))
          (if (== (Variables|Default|GetHit%20Counter) 2) :!label _label
            (Variables|Default|SetHit%20Counter 0)
            (else
              (Variables|Default|SetHit%20Counter (+ (Variables|Default|GetHit%20Counter) 1))
              ;[0.15 0.15 0.15 0.5] Health Logic
              (CallFunction|UpdateCurrentHealth Damage)
              (CallFunction|UpdateHealthbar)
              ;[0.15 0.15 0.15 0.5] Check if possessed armour is dead
              (if (<= (Variables|Default|GetCurrent_Health) 0.0)
                (Actor|DestroyActor)))))
        (else
          (goto _label))))))

(fn ConstructionScript)

(fn UpdateHealthbar
  (bind _aswbp_healthbar_skeleton (Utilities|Casting|CastToWBP_Healthbar_Skeleton (UserInterface|GetUserWidgetObject (Variables|Default|GetHealthbar))))
  (bind _output_get (Variables|Default|SetAs%20WBP%20Healthbar _aswbp_healthbar_skeleton))
  (Variables|/Game/Blueprints/Enemies/Skeletons/WBP_Healthbar_Skeleton.WBP_Healthbar_Skeleton_C|SetCurrent%20Health _output_get (Variables|Default|GetCurrent_Health))
  (Variables|/Game/Blueprints/Enemies/Skeletons/WBP_Healthbar_Skeleton.WBP_Healthbar_Skeleton_C|SetMax%20Health _output_get (Variables|Default|GetMax_Health)))

(fn UpdateCurrentHealth
  (params (Damage :type Float%20%28double-precision%29))
  ;[0.15 0.15 0.15 0.5] Update Current Health
  (Variables|Default|SetCurrent_Health (- (Variables|Default|GetCurrent_Health) Damage)))