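; BP_Weapon_Stats defines the stats for the game's weapons: Fists, Sword, Axe, Bow, Shield and Plumbata.
; On BeginPlay it packs individual per-weapon variables into named melee, ranged or defense structs, stored in one variable per weapon.
; Each weapon fills only relevant fields, so Fists has no durability, only the Axe sets enemy stun and only the Bow sets charge-up values.
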(event EventBeginPlay
  (Variables|Fists|SetFists_Stats (Utilities|Struct|MakeStruct_Melee_Weapon_Stats (Variables|Fists|GetFists_Damage) (Variables|Fists|GetFists_AttackRange) (Variables|Fists|GetFists_AttackPerSecond) (Variables|Fists|GetFists_AnimationDuration) (Variables|Fists|GetFists_Cooldown) (Variables|Fists|GetFists_StaminaUsage) 0.0 0.0 "Fists"))
  (Variables|Sword|SetSword_Stats (Utilities|Struct|MakeStruct_Melee_Weapon_Stats (Variables|Sword|GetSword_Damage) (Variables|Sword|GetSword_AttackRange) (Variables|Sword|GetSword_AttackPerSecond) (Variables|Sword|GetSword_AnimationDuration) (Variables|Sword|GetSword_Cooldown) (Variables|Sword|GetSword_StaminaUsage) (Variables|Sword|GetSword_Durability) 0.0 "Sword"))
  (Variables|Axe|SetAxe_Stats (Utilities|Struct|MakeStruct_Melee_Weapon_Stats (Variables|Axe|GetAxe_Damage) (Variables|Axe|GetAxe_AttackRange) (Variables|Axe|GetAxe_AttackPerSecond) (Variables|Axe|GetAxe_AnimationDuration) (Variables|Axe|GetAxe_Cooldown) (Variables|Axe|GetAxe_StaminaUsage) (Variables|Axe|GetAxe_Durability) (Variables|Axe|GetAxe_EnemyStun) "Axe"))
  (Variables|Bow|SetBow_Stats (Utilities|Struct|MakeStruct_Ranged_Weapon_Stats (Variables|Bow|GetBow_Damage) (Variables|Bow|GetBow_Range) (Variables|Bow|GetBow_ChargeUpRange) (Variables|Bow|GetBow_ProjectileSpeed) (Variables|Bow|GetBow_ChargeUpTime) (Variables|Bow|GetBow_StaminaUsage) (Variables|Bow|GetBow_Cooldown) (Variables|Bow|GetBow_Durability) 0.0 "Bow"))
  (Variables|Shield|SetShield_Stats (Utilities|Struct|MakeStruct_Defense_Weapon_Stats (Variables|Shield|GetShield_DamageBlocked) (Variables|Shield|GetShield_AnimationDuration) (Variables|Shield|GetShield_StaminaUsage) (Variables|Shield|GetShield_Cooldown) (Variables|Shield|GetShield_Durability) "Shield"))
  (Variables|Plumbata|SetPlumbata_Stats (Utilities|Struct|MakeStruct_Ranged_Weapon_Stats (Variables|Plumbata|GetPlumbata_Damage) (Variables|Plumbata|GetPlumbata_Range) 0.0 (Variables|Plumbata|GetPlumbata_ProjectileSpeed) 0.0 (Variables|Plumbata|GetPlumbata_StaminaUsage) (Variables|Plumbata|GetPlumbata_Cooldown) (Variables|Plumbata|GetPlumbata_Durability) (Variables|Plumbata|GetPlumbata_AnimationDuration) "Plumbata")))