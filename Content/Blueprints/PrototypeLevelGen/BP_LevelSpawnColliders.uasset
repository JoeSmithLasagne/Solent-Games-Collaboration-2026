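; BP_LevelSpawnColliders provides north, south, east and west door triggers that load the next level in the prototype level generation.
; Any door overlap, with no check on the overlapping actor, calls LoadNextLevel on BP_MainGameInstance, passing its parent actor as the current level and a stored spawn location and rotation.
; TransformPlayerPos sets that shared spawn from a given component's world transform; nothing in this Blueprint calls it.
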(event OnComponentBeginOverlap(EastDoorCollider)
  (params (OverlappedComponent :type Primitive%20Component%20Object%20Reference) (OtherActor :type Actor%20Object%20Reference) (OtherComp :type Primitive%20Component%20Object%20Reference) (OtherBodyIndex :type Integer) (bFromSweep :type Boolean) (SweepResult :type Hit%20Result%20Structure%20%28by%20ref%29))
  (bind _asbp_main_game_instance (Utilities|Casting|CastToBP_MainGameInstance (Game|GetGameInstance)))
  (Default|LoadNextLevel _asbp_main_game_instance 0 (Actor|GetParentActor) (Variables|Default|GetPlayerSpawnVector) (Variables|Default|GetPlayerSpawnRot)))

(event OnComponentBeginOverlap(WestDoorCollider)
  (params (OverlappedComponent :type Primitive%20Component%20Object%20Reference) (OtherActor :type Actor%20Object%20Reference) (OtherComp :type Primitive%20Component%20Object%20Reference) (OtherBodyIndex :type Integer) (bFromSweep :type Boolean) (SweepResult :type Hit%20Result%20Structure%20%28by%20ref%29))
  (bind _asbp_main_game_instance (Utilities|Casting|CastToBP_MainGameInstance (Game|GetGameInstance)))
  (Default|LoadNextLevel _asbp_main_game_instance 0 (Actor|GetParentActor) (Variables|Default|GetPlayerSpawnVector) (Variables|Default|GetPlayerSpawnRot)))

(event OnComponentBeginOverlap(SouthDoorCollider)
  (params (OverlappedComponent :type Primitive%20Component%20Object%20Reference) (OtherActor :type Actor%20Object%20Reference) (OtherComp :type Primitive%20Component%20Object%20Reference) (OtherBodyIndex :type Integer) (bFromSweep :type Boolean) (SweepResult :type Hit%20Result%20Structure%20%28by%20ref%29))
  (bind _asbp_main_game_instance (Utilities|Casting|CastToBP_MainGameInstance (Game|GetGameInstance)))
  (Default|LoadNextLevel _asbp_main_game_instance 0 (Actor|GetParentActor) (Variables|Default|GetPlayerSpawnVector) (Variables|Default|GetPlayerSpawnRot)))

(event OnComponentBeginOverlap(NorthDoorCollider)
  (params (OverlappedComponent :type Primitive%20Component%20Object%20Reference) (OtherActor :type Actor%20Object%20Reference) (OtherComp :type Primitive%20Component%20Object%20Reference) (OtherBodyIndex :type Integer) (bFromSweep :type Boolean) (SweepResult :type Hit%20Result%20Structure%20%28by%20ref%29))
  (bind _asbp_main_game_instance (Utilities|Casting|CastToBP_MainGameInstance (Game|GetGameInstance)))
  (Default|LoadNextLevel _asbp_main_game_instance 0 (Actor|GetParentActor) (Variables|Default|GetPlayerSpawnVector) (Variables|Default|GetPlayerSpawnRot)))

(fn ConstructionScript)

(fn TransformPlayerPos
  (params (PlayerTransformPos :type Capsule%20Component%20Object%20Reference))
  (Variables|Default|SetPlayerSpawnVector (Transformation|GetWorldLocation PlayerTransformPos))
  (Variables|Default|SetPlayerSpawnRot (Transformation|GetWorldRotation PlayerTransformPos))
  (return))