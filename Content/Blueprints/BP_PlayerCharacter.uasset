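; Player character with camera-relative movement, a stamina-costed dodge roll, health and an in-game HUD.
; Tick regenerates stamina and drives the timed roll, which raises walk speed along the last input direction, or mesh forward if none, then starts a cooldown.
; Rolling blocks damage, self-inflicted damage is ignored, and death currently just resets health.
; A bound dispatcher event destroys passed-in hitbox components.
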(event Custom|DestoryComponent_Event
  (params (NewParam :type Actor%20Component%20Object%20Reference))
  ;[0.15 0.15 0.15 0.5] Destroy hitbox
  (Components|DestroyComponent NewParam))

(event EventTick
  (params (DeltaSeconds :type Float%20%28single-precision%29))
  (bind _charactermovement (Variables|Character|GetCharacterMovement))
  (bind _stamina (Variables|Default|GetStamina))
  (Utilities|FlowControl|Sequence
    (:then_0
      ;[0.15 0.15 0.15 0.5] Stamina Regen
      (if (>= (- (Utilities|Time|GetTimeSeconds) (Variables|Default|GetStaminaRegenLastTime)) (Variables|Default|GetStaminRegenRate))
        (if (< _stamina (Variables|Default|GetMaxStamina))
          (CallFunction|RegenStamina)
          (Variables|Default|SetStaminaRegenLastTime (Utilities|Time|GetTimeSeconds))
          (Development|PrintString (Utilities|String|ToString(Float) _stamina)))))
    (:then_1
      ;[0.15 0.15 0.15 0.5] Check if Player is Rolling
      (if (Variables|Default|GetIsRolling)
        ;[0.15 0.15 0.15 0.5] End Roll if duration is met or exceeded
        (if (>= (- (Utilities|Time|GetTimeSeconds) (Variables|Default|GetRollStartTime)) (Variables|Default|GetRollDurationSeconds))
          (Variables|Default|SetIsRolling false)
          (Variables|Default|SetRollCooldownStartTime (Utilities|Time|GetTimeSeconds))
          (Variables|/Script/Engine.CharacterMovementComponent|SetMaxWalkSpeed (Variables|Character|GetCharacterMovement) (Variables|Default|GetMaxMoveSpeed))
          (else
            ;[0.15 0.15 0.15 0.5] Roll while rolling state is active (if input direction is empty (0) we just go in the player's view direction)
            (if (Utilities|Operators|EqualEqual :A (Variables|Default|GetMovementDirection))
              (Class|PawnMovementComponent|AddInputVector _charactermovement (Math|Vector|GetForwardVector (Transformation|GetWorldRotation (Variables|Character|GetMesh))) false)
              (else
                (Class|PawnMovementComponent|AddInputVector _charactermovement (Variables|Default|GetMovementDirection) false)))))))))

(event EventBeginPlay
  ;[0.15 0.15 0.15 0.5] Destroy hitbox
  (EventDispatchers|BindEventtoDestoryComponent (delegate Custom|DestoryComponent_Event))
  ;[0.15 0.15 0.15 0.5] Initialise Stats
  (Variables|Default|SetStamina (Variables|Default|GetMaxStamina))
  (Variables|Default|SetHealth (Variables|Default|GetMaxHealth))
  (bind _returnvalue (UserInterface|CreateWidget "/Game/Blueprints/Widgets/InGameUi/InGameHud.InGameHud_C"))
  (bind _output_get (Variables|Default|SetHUDRef _returnvalue))
  (UserInterface|Viewport|AddtoViewport _output_get 0))

(event Game|Damage|EventAnyDamage
  (params (Damage :type Float%20%28single-precision%29) (DamageType :type Damage%20Type%20Object%20Reference) (InstigatedBy :type Controller%20Object%20Reference) (DamageCauser :type Actor%20Object%20Reference))
  ;[0.15 0.15 0.15 0.5] Take damage so long as the inflictor isn't the player themself
  (if (not (== DamageCauser self))
    (CallFunction|TakeDamage Damage)))

(event Input|ActionEvents|InputActionRoll
  (params (Key :type Key%20Structure :default "None"))
  ;[0.15 0.15 0.15 0.5] Toggle Roll
  (:Pressed
    (if (not (Variables|Default|GetIsRolling))
      (if (>= (- (Utilities|Time|GetTimeSeconds) (Variables|Default|GetRollCooldownStartTime)) (Variables|Default|GetRoolCooldown))
        (if (>= (Variables|Default|GetStamina) (Variables|Default|GetRollStaminaCost))
          (Variables|Default|SetStamina (- (Variables|Default|GetStamina) (Variables|Default|GetRollStaminaCost)))
          (Variables|Default|SetIsRolling true)
          (Variables|Default|SetRollStartTime (Utilities|Time|GetTimeSeconds))
          (Variables|/Script/Engine.CharacterMovementComponent|SetMaxWalkSpeed (Variables|Character|GetCharacterMovement) (Variables|Default|GetRollSpeed)))))))

(event Input|AxisEvents|InputAxisMoveForward
  (params (AxisValue :type Float%20%28single-precision%29))
  (bind _returnvalue (Input|AxisValues|GetMoveForward))
  (bind _camera (Variables|Default|GetCamera))
  (bind _returnvalue_2 (Transformation|GetWorldRotation _camera))
  (bind _returnvalue_3 (Math|Vector|GetForwardVector (Math|Rotator|MakeRotator 0.0 0.0 (.yaw _returnvalue_2))))
  (bind _returnvalue_4 (* _returnvalue_3 _returnvalue))
  ;[0.15 0.15 0.15 0.5] Horizontal Movement
  (if (not (Variables|Default|GetIsRolling))
    (Class|PawnMovementComponent|AddInputVector (Variables|Character|GetCharacterMovement) _returnvalue_4 false)
    (Variables|Default|SetMovementDirection (+ _returnvalue_4 (* (Math|Vector|GetRightVector (Math|Rotator|MakeRotator 0.0 0.0 (.yaw _returnvalue_2))) (Input|AxisValues|GetMoveRight))))))

(event Input|AxisEvents|InputAxisMoveRight
  (params (AxisValue :type Float%20%28single-precision%29))
  (bind _returnvalue (Input|AxisValues|GetMoveRight))
  (bind _camera (Variables|Default|GetCamera))
  (bind _returnvalue_2 (Transformation|GetWorldRotation _camera))
  (bind _returnvalue_3 (Math|Vector|GetRightVector (Math|Rotator|MakeRotator 0.0 0.0 (.yaw _returnvalue_2))))
  (bind _returnvalue_4 (* _returnvalue_3 _returnvalue))
  ;[0.15 0.15 0.15 0.5] Horizontal Movement
  (if (not (Variables|Default|GetIsRolling))
    (Class|PawnMovementComponent|AddInputVector (Variables|Character|GetCharacterMovement) _returnvalue_4 false)
    (Variables|Default|SetMovementDirection (+ (* (Math|Vector|GetForwardVector (Math|Rotator|MakeRotator 0.0 0.0 (.yaw _returnvalue_2))) (Input|AxisValues|GetMoveForward)) _returnvalue_4))))

(fn ConstructionScript)

(fn TakeDamage
  (params (Damage :type Float%20%28double-precision%29))
  (if (not (Variables|Default|GetIsRolling))
    (bind _output_get (Variables|Default|SetHealth (- (Variables|Default|GetHealth) Damage)))
    (if (<= _output_get 0.0)
      (CallFunction|KIllPlayer)
      (else
        (Development|PrintString (Utilities|String|ToString(Float) _output_get))
        (Development|PrintString "Player took damage")))))

(fn KIllPlayer
  (Development|PrintString "Player Died")
  (Variables|Default|SetHealth (Variables|Default|GetMaxHealth)))

(fn HealPlayer
  (params (Healing :type Float%20%28double-precision%29))
  (bind _output_get (Variables|Default|SetHealth (Math|Float|Clamp(Float) (+ Healing (Variables|Default|GetHealth)) 0.0 (Variables|Default|GetMaxHealth))))
  (Development|PrintString (Utilities|String|ToString(Float) _output_get))
  (Development|PrintString "Player Healed"))

(fn RegenStamina
  (bind _maxstamina (Variables|Default|GetMaxStamina))
  (if (> (+ (Variables|Default|GetStamina) (Variables|Default|GetStaminaRegenAmount)) _maxstamina)
    (Variables|Default|SetStamina _maxstamina)
    (else
      (Variables|Default|SetStamina (+ (Variables|Default|GetStamina) (Variables|Default|GetStaminaRegenAmount))))))