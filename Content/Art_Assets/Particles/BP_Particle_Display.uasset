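; BP_Particle_Display is an actor that repeatedly spawns a configurable Particle actor class at its own transform, apparently to showcase effects.
; Tick accumulates delta time and, once it reaches Frequency, subtracts that interval and spawns a new instance regardless of collision.
; Each spawned actor receives the configured Lifespan, so it removes itself without further tracking.
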(event EventBeginPlay)

(event Collision|EventActorBeginOverlap
  (params (OtherActor :type Actor%20Object%20Reference)))

(event EventTick
  (params (DeltaSeconds :type Float%20%28single-precision%29))
  (bind _frequency (Variables|Stats|GetFrequency))
  (bind _output_get (Variables|Logic|SetTime (+ DeltaSeconds (Variables|Logic|GetTime))))
  (if (>= _output_get _frequency)
    (Variables|Logic|SetTime (- (Variables|Logic|GetTime) _frequency))
    (bind _returnvalue (Game|SpawnActorfromClass (Variables|Stats|GetParticle) (Transformation|GetActorTransform) "AlwaysSpawn" "MultiplyWithRoot" 0 0))
    (Actor|SetLifeSpan _returnvalue (Variables|Stats|GetLifespan))))

(fn ConstructionScript)