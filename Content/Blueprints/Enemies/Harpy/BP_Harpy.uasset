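; Harpy enemy that loses health only to ranged damage and destroys itself at zero, updating a healthbar widget.
; A DoOnce gate, reset from Tick after a delay, provides immunity frames between hits.
; Slash damages the player directly; dash lerps forward on a timeline, damaging every update once an overlap sets OverlapPlayer, which never clears.
; Pickup and feather attacks are empty stubs, and debug prints remain.
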(event Custom|Dash%20Attack
  (Development|PrintString "Dash attack")
  (CallFunction|MoveOverTime (+ (Transformation|GetActorLocation) (* (Math|Vector|GetForwardVector (Transformation|GetActorRotation)) 6e+02))))

(event Custom|Pickup%20Attack)

(event Custom|Feather%20Attack)

(event Custom|Slash%20Attack
  ;[0.15 0.15 0.15 0.5] Attack debug
  (Development|PrintString "Attacking")
  ;[0.15 0.15 0.15 0.5] Apply Damage
  (Game|Damage|ApplyDamage (Game|GetPlayerCharacter 0) (Variables|Default|GetSlashAttack_Damage) 0 self))

(event Custom|MoveOverTime
  (params (End%20Location :type Vector))
  (Variables|Default|SetDash_Start_Location (Transformation|GetActorLocation))
  (bind _dashtrack (Timeline|DashTimeline PlayFromStart)
    (:Update
      (Transformation|SetActorLocation (Math|Vector|Lerp(Vector) (Variables|Default|GetDash_Start_Location) End%20Location _dashtrack) false true)
      (if (Variables|Default|GetOverlapPlayer)
        (Game|Damage|ApplyDamage (Game|GetPlayerCharacter 0) (Variables|Default|GetDashAttack_Damage) 0 self)
        (Development|PrintString "Damaging")))))

(event Custom|OnActorBeginOverlap_Event
  (params (OverlappedActor :type Actor%20Object%20Reference) (OtherActor :type Actor%20Object%20Reference))
  (Utilities|Casting|CastToBP_PlayerCharacter OtherActor)
  (Variables|Default|SetOverlapPlayer true))

(event EventTick
  (params (DeltaSeconds :type Float%20%28single-precision%29))
  ;[0.15 0.15 0.15 0.5] Immunity Frames
  (if (Variables|Default|GetHit)
    (Utilities|FlowControl|Delay (Variables|Default|GetImmunity_Frames))
    (Variables|Default|SetHit false)
    (Utilities|FlowControl|DoOnce false) ; enters at Reset
  ))

(event EventBeginPlay
  ;[0.15 0.15 0.15 0.5] Set movement speed
  (Variables|/Script/Engine.CharacterMovementComponent|SetMaxWalkSpeed (Variables|Character|GetCharacterMovement) (Variables|Default|GetMovement_Speed))
  ;[0.15 0.15 0.15 0.5] Set current health
  (Variables|Default|SetCurrent_Health (Variables|Default|GetMax_Health))
  (CallFunction|UpdateHealthbar))

(event Game|Damage|EventAnyDamage
  (params (Damage :type Float%20%28single-precision%29) (DamageType :type Damage%20Type%20Object%20Reference) (InstigatedBy :type Controller%20Object%20Reference) (DamageCauser :type Actor%20Object%20Reference))
  ;[0.15 0.15 0.15 0.5] Immunity Frames
  (Utilities|FlowControl|DoOnce false
    (:Completed
      (Variables|Default|SetHit true)
      (if (Utilities|Enum|Equal(Enum) (Variables|Default|GetDamage_Type) "Ranged")
        ;[0.15 0.15 0.15 0.5] Health Logic
        (CallFunction|UpdateCurrentHealth Damage)
        (CallFunction|UpdateHealthbar)
        ;[0.15 0.15 0.15 0.5] Check if harpy is dead
        (if (<= (Variables|Default|GetCurrent_Health) 0.0)
          (Actor|DestroyActor))))))

(fn ConstructionScript)

(fn UpdateHealthbar
  (bind _aswbp_healthbar_skeleton (Utilities|Casting|CastToWBP_Healthbar_Skeleton (UserInterface|GetUserWidgetObject (Variables|Default|GetHealthbar))))
  (bind _output_get (Variables|Default|SetAs%20WBP%20Healthbar _aswbp_healthbar_skeleton))
  (Variables|/Game/Blueprints/Enemies/Skeletons/WBP_Healthbar_Skeleton.WBP_Healthbar_Skeleton_C|SetCurrent%20Health _output_get (Variables|Default|GetCurrent_Health))
  (Variables|/Game/Blueprints/Enemies/Skeletons/WBP_Healthbar_Skeleton.WBP_Healthbar_Skeleton_C|SetMax%20Health _output_get (Variables|Default|GetMax_Health)))

(fn UpdateCurrentHealth
  (params (Damage :type Float%20%28double-precision%29))
  ;[0.15 0.15 0.15 0.5] Update Current Health
  (Variables|Default|SetCurrent_Health (- (Variables|Default|GetCurrent_Health) Damage)))