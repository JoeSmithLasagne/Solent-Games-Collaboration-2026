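; BP_Item is a pickup actor that previews its item's mesh in the construction script, then spins and bobs it during play.
; Sphere overlaps toggle a prompt widget and weapon-details notifications, filtered by slot type and mesh.
; Pressing F shows a taken notification and activates the Sphere, whose activation event drives a timeline lifting the actor with Niagara effects before destroying it.
; No inventory transfer happens here.
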(event OnComponentBeginOverlap(Sphere)
  (params (OverlappedComponent :type Primitive%20Component%20Object%20Reference) (OtherActor :type Actor%20Object%20Reference) (OtherComp :type Primitive%20Component%20Object%20Reference) (OtherBodyIndex :type Integer) (bFromSweep :type Boolean) (SweepResult :type Hit%20Result%20Structure%20%28by%20ref%29))
  (bind _item (Variables|Default|GetItem))
  (bind (_slottype _item_2) (Utilities|Struct|BreakS_EquipmentSlot _item))
  ;[0.15 0.15 0.15 0.5] Taking Items Interaction
  (Utilities|FlowControl|Sequence
    (:then_0
      (if (Utilities|Enum|Equal(Enum) _slottype "NewEnumerator0")
        (if (== (.Mesh (Utilities|Struct|BreakS_ItemStructure _item_2)) 0) :!label _label
          (Default|WeaponNotification (Variables|Default|GetWeaponWidget))
          (Rendering|SetVisibility (Variables|Default|GetWidget) true false))))
    (:then_1
      (if (Utilities|Enum|Equal(Enum) _slottype "NewEnumerator1")
        (goto _label)))
    (:then_2
      (if (Utilities|Enum|Equal(Enum) _slottype "NewEnumerator2")
        (goto _label)))))

(event OnComponentActivated(Sphere)
  (params (Component :type Actor%20Component%20Object%20Reference) (bReset :type Boolean))
  ;[0.15 0.15 0.15 0.5] Item Animation
  (Input|EnableInput (Game|GetPlayerController 0))
  (Utilities|FlowControl|Delay 0.2)
  (bind _output_get (Variables|Default|SetStartLocation (Transformation|GetActorLocation)))
  (bind _alpha1 (Timeline|Timeline Play)
    (:Update
      (Transformation|SetActorLocation (Math|Vector|Lerp(Vector) _output_get (+ _output_get "0.000000,0.000000,300.000000") _alpha1) false false)
      (Niagara|SpawnSystematLocation "/Game/Blueprints/Animations/Movement_Efffects/NiagaraRegular.NiagaraRegular" (Math|Vector|Lerp(Vector) _output_get (+ _output_get "0.000000,0.000000,300.000000") _alpha1))
      (Utilities|FlowControl|Delay 2.0)
      (Actor|DestroyActor))))

(event OnComponentEndOverlap(Sphere)
  (params (OverlappedComponent :type Primitive%20Component%20Object%20Reference) (OtherActor :type Actor%20Object%20Reference) (OtherComp :type Primitive%20Component%20Object%20Reference) (OtherBodyIndex :type Integer))
  ;[0.15 0.15 0.15 0.5] Taking Items Interaction
  (Input|DisableInput 0)
  (Default|WeaponNotificationOut (Variables|Default|GetWeaponWidget))
  (Rendering|SetVisibility (Variables|Default|GetWidget) false false))

(event Custom|Animate%20Boxes
  ;[0.15 0.15 0.15 0.5] Object Animation (Not Taken)
  (bind _alpha (Timeline|Object%20Movement PlayFromStart)
    (:Update
      (Transformation|SetRelativeLocation (Variables|Default|GetStaticMesh) (Math|Vector|MakeVector 0.0 0.0 _alpha) false false))))

(event EventBeginPlay
  ;[0.15 0.15 0.15 0.5] Object Animation (Not Taken)
  (CallFunction|AnimateBoxes)
  ;;[0.15 0.15 0.15 0.5] Object --> Deactivated at the beginning of the Program
  (Components|Activation|Deactivate (Variables|Default|GetSphere))
  (bind _returnvalue (UserInterface|CreateWidget "/Game/Inventory/Blueprints/Widget_Animations/WB_WeaponDetails.WB_WeaponDetails_C"))
  (bind _output_get (Variables|Default|SetWeaponWidget _returnvalue))
  (UserInterface|Viewport|AddtoViewport _output_get 0))

(event Collision|EventActorBeginOverlap
  (params (OtherActor :type Actor%20Object%20Reference)))

(event EventTick
  (params (DeltaSeconds :type Float%20%28single-precision%29))
  ;[0.15 0.15 0.15 0.5] Object Animation (Not Taken)
  (Transformation|AddLocalRotation (Variables|Default|GetStaticMesh) "0.000000,0.500000,0.000000" false false))

(event Input|KeyboardEvents|F
  (params (Key :type Key%20Structure :default "None"))
  ;[0.15 0.15 0.15 0.5] Item Animation
  (:Pressed
    (Default|WeaponTakenNotification (Variables|Default|GetWeaponWidget))
    (Components|Activation|Activate (Variables|Default|GetSphere) false)))

(fn ConstructionScript
  ;[0.15 0.15 0.15 0.5] Construction Script to see the Item already build before executing the Level
  (Components|StaticMesh|SetStaticMesh (Variables|Default|GetStaticMesh) (.mesh (.Item (Utilities|Struct|BreakS_EquipmentSlot (Variables|Default|GetItem)))))
  (Physics|SetSimulatePhysics (Variables|Default|GetStaticMesh) false))