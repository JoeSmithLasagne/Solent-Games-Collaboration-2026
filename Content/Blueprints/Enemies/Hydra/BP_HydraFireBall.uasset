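; Hydra enemy fireball actor that can burst into a ring of further fireballs.
; A timer set from Lifetime at BeginPlay calls Explode, and a sphere collider overlap cancels it to explode immediately.
; When DoExplosion is set, Explode spawns eight evenly yawed copies with Parent as instigator, calling SetStats on each without passing values.
; SetStats stores damage, lifetime, explosion flag and parent; the graphs neither apply damage nor destroy the actor.
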(event OnComponentBeginOverlap(Sphere_Collider)
  (params (OverlappedComponent :type Primitive%20Component%20Object%20Reference) (OtherActor :type Actor%20Object%20Reference) (OtherComp :type Primitive%20Component%20Object%20Reference) (OtherBodyIndex :type Integer) (bFromSweep :type Boolean) (SweepResult :type Hit%20Result%20Structure%20%28by%20ref%29))
  (Utilities|Time|ClearandInvalidateTimerbyHandle (Variables|Default|GetExplodeTimer))
  (CallFunction|Explode))

(event EventBeginPlay
  (bind _returnvalue (Utilities|Time|SetTimerbyFunctionName 0 "Explode" (Variables|Default|GetLifetime)))
  (Variables|Default|SetExplodeTimer _returnvalue))

(fn ConstructionScript)

(fn SetStats
  (params (Damage :type Float%20%28double-precision%29) (LifeTime :type Float%20%28double-precision%29) (DoExplosion :type Boolean) (Parent :type Pawn%20Object%20Reference))
  (Variables|Default|SetDamage Damage)
  (Variables|Default|SetLifetime LifeTime)
  (Variables|Default|SetDoExplosion DoExplosion)
  (Variables|Default|SetParent Parent))

(fn Explode
  (bind _returnvalue (Transformation|GetActorTransform))
  (if (Variables|Default|GetDoExplosion)
    (for _index (range 0 7)
      (bind _returnvalue_2 (Game|SpawnActorfromClass "BP_HydraFireBall_C" (Math|Transform|MakeTransform (.location _returnvalue) (Class|KismetMathLibrary|QuatRotator (* (Math|Conversions|ToQuaternion(Rotator) (Math|Rotator|MakeRotator 0.0 0.0 (* _index 45.0))) (Math|Conversions|ToQuaternion(Rotator) (.rotation _returnvalue)))) (.scale _returnvalue)) "Undefined" "MultiplyWithRoot" 0 (Variables|Default|GetParent)))
      (CallFunction|SetStats _returnvalue_2 0.0 0.0 false))))