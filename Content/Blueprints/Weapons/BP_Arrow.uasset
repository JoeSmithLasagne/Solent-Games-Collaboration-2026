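; BP_Arrow is a projectile weapon actor that covers regular arrows, charged arrows and a plumbata variant.
; Its construction script sets the projectile speed and derives a lifetime from the range for the active variant divided by that speed.
; A timer destroys the arrow when that lifetime ends, and the cylinder's overlap applies damage to any actor other than the first player character, without destroying the arrow.
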(event OnComponentBeginOverlap(Cylinder)
  (params (OverlappedComponent :type Primitive%20Component%20Object%20Reference) (OtherActor :type Actor%20Object%20Reference) (OtherComp :type Primitive%20Component%20Object%20Reference) (OtherBodyIndex :type Integer) (bFromSweep :type Boolean) (SweepResult :type Hit%20Result%20Structure%20%28by%20ref%29))
  (if (not (== OtherActor (Game|GetPlayerCharacter 0)))
    (Game|Damage|ApplyDamage OtherActor (Variables|Default|GetDamage) 0 0)))

(event Custom|Destroy%20Arrow
  (Actor|DestroyActor))

(event EventBeginPlay
  (Utilities|Time|SetTimerbyEvent (delegate Custom|Destroy%20Arrow) (Variables|Default|GetLifetime)))

(event Collision|EventActorBeginOverlap
  (params (OtherActor :type Actor%20Object%20Reference)))

(event EventTick
  (params (DeltaSeconds :type Float%20%28single-precision%29)))

(fn ConstructionScript
  (bind _projectilespeed (Variables|Default|GetProjectileSpeed))
  (Variables|/Script/Engine.ProjectileMovementComponent|SetInitialSpeed (Variables|Default|GetProjectileMovement) (Variables|Default|GetProjectileSpeed))
  (if (Variables|Default|GetIsPlumbata)
    (Variables|Default|SetLifetime (/ (Variables|Default|GetPlumbataRange) _projectilespeed))
    (elif (Variables|Default|GetCharged)
      (Variables|Default|SetLifetime (/ (Variables|Default|GetArrowChargedRange) _projectilespeed))
      (else
        (Variables|Default|SetLifetime (/ (Variables|Default|GetArrowRange) _projectilespeed))))))