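; Shielded skeleton enemy that blocks incoming hits until its shield breaks, and deals damage to the player through an Attack event.
; Damage passes an immunity-frame gate, then either uses up a block charge or, with the shield broken, reduces health, updates the healthbar widget and destroys the actor at zero.
; Delays and a second DoOnce restore block charges after the break window lapses or the broken-shield cooldown ends.
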(event Custom|Immunity%20Frames%20Finished
  ;[1 1 1 0.502] Immunity Frames
  (Utilities|FlowControl|DoOnce false) ; enters at Reset
)

(event Custom|Attack
  ;[0 0 0] Debug
  (Development|PrintString "Attacking")
  ;[0 1 0] Damage To Do!
  (Game|Damage|ApplyDamage (Game|GetPlayerCharacter 0) (Variables|Stats|GetAttack_Damage) 0 self))

(event EventBeginPlay
  ;[0.15 0.15 0.6514 0.502] Setting Movement Speed
  (Variables|/Script/Engine.CharacterMovementComponent|SetMaxWalkSpeed (Variables|Character|GetCharacterMovement) (Variables|Stats|GetMovement_Speed))
  ;[0.15 0.04092 0.02843 0.502] Setting Current Health To Max Health
  (Variables|Stats|SetCurrent_Health (Variables|Stats|GetMax_Health))
  (CallFunction|UpdateHealthbar)
  ;[0 0.145 0.15 0.5] Set up for shield breaking logic
  (Variables|Default|SetRemaining%20hits (Variables|Stats|GetHits%20To%20Break%20Shield)))

(event Game|Damage|EventAnyDamage
  (params (Damage :type Float%20%28single-precision%29) (DamageType :type Damage%20Type%20Object%20Reference) (InstigatedBy :type Controller%20Object%20Reference) (DamageCauser :type Actor%20Object%20Reference))
  ;[1 1 1 0.502] Immunity Frames
  (Utilities|FlowControl|DoOnce false
    (:Completed
      (Utilities|Time|SetTimerbyFunctionName 0 "Immunity Frames Finished" (Variables|Stats|GetImmunity_Frames_Timer))
      ;[0 0.15 0.139 0.5] Shield Logic
      (if (<= (Variables|Default|GetRemaining%20hits) 0)
        ;[0.15 0.02315 0.02956 0.502] Health Logic
        (CallFunction|UpdateCurrentHealth Damage)
        (CallFunction|UpdateHealthbar)
        ;[0.15 0.15 0.15 0.502] Check If Skeleton Is Dead
        (if (<= (Variables|Stats|GetCurrent_Health) 0.0)
          (Actor|DestroyActor))
        (else
          ;[0 0.15 0.139 0.5] Shield Logic
          ;;[0.07955 0.07925 0.15 0.5] Decrease hits to break by 1
          (Variables|Default|SetRemaining%20hits (- (Variables|Default|GetRemaining%20hits) 1))
          (if (<= (Variables|Default|GetRemaining%20hits) 0)
            _
            (else
              ;;[0.15 0.001653 7e-06 0.5] Timer for window needed to break the shield before restoring block charges
              (Utilities|FlowControl|Delay (Variables|Stats|GetShield%20Break%20Window%20Time))))
          (Utilities|FlowControl|DoOnce false :!label _label
            (:Completed
              (if (<= (Variables|Default|GetRemaining%20hits) 0)
                ;;[0.15 0.00217 0 0.5] Timer for cooldown if shield has been broken
                (Utilities|FlowControl|Delay (Variables|Stats|GetShield%20Cooldown)))
              ;;[0.05779 0.15 0.07598 0.5] Reset hits to break
              (Variables|Default|SetRemaining%20hits (Variables|Stats|GetHits%20To%20Break%20Shield))
              (goto _label Reset))))))))

(fn ConstructionScript)

(fn UpdateHealthbar
  (bind _aswbp_healthbar_skeleton (Utilities|Casting|CastToWBP_Healthbar_Skeleton (UserInterface|GetUserWidgetObject (Variables|Default|GetHealthbar))))
  (bind _output_get (Variables|Default|SetAs%20WBP%20Healthbar%20Skeleton _aswbp_healthbar_skeleton))
  ;[0.15 0.1222 0.05534 0.5] Set helth variables in the healthbar function
  (Variables|/Game/Blueprints/Enemies/Skeletons/WBP_Healthbar_Skeleton.WBP_Healthbar_Skeleton_C|SetCurrent%20Health _output_get (Variables|Stats|GetCurrent_Health))
  (Variables|/Game/Blueprints/Enemies/Skeletons/WBP_Healthbar_Skeleton.WBP_Healthbar_Skeleton_C|SetMax%20Health _output_get (Variables|Stats|GetMax_Health)))

(fn UpdateCurrentHealth
  (params (Damage :type Float%20%28double-precision%29))
  ;[0.15 0.0156 0.004484 0.5] Update Current Health
  (Variables|Stats|SetCurrent_Health (- (Variables|Stats|GetCurrent_Health) Damage)))