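; Base Chimera boss character with bite, venom spit and charge attacks, whose health drives the player HUD's boss bar.
; BeginPlay scales health and damage by a multiplier.
; Attack, Shoot, Charge and Rotate are callable events, with DoOnce-plus-Delay cooldowns on attacks, damage passed to spawned spit via ApplyDamage, and charge hits from box overlap.
; Tick polls health for death, toggling the bar, playing audio and destroying the actor.
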(event OnComponentBeginOverlap(Box)
  (params (OverlappedComponent :type Primitive%20Component%20Object%20Reference) (OtherActor :type Actor%20Object%20Reference) (OtherComp :type Primitive%20Component%20Object%20Reference) (OtherBodyIndex :type Integer) (bFromSweep :type Boolean) (SweepResult :type Hit%20Result%20Structure%20%28by%20ref%29))
  ;[0.15 0.15 0.15 0.5] Charge Attack with damage and trigger
  (if (Variables|Default|GetCanCharge)
    (Utilities|FlowControl|DoOnce false :!label _label
      (:Completed
        (Development|PrintString "ChimeraChargeHit")
        (Game|Damage|ApplyDamage (Game|GetPlayerCharacter 0) (Variables|Default|GetChargeAttackDamage) 0 0)
        (Utilities|FlowControl|Delay (Variables|Default|GetChargeAttackSpeed))
        (goto _label Reset)))))

(event Custom|Attack
  (bind _arrow1 (Variables|Default|GetArrow1))
  (bind _returnvalue (Transformation|GetWorldLocation _arrow1))
  ;[0.15 0.15 0.15 0.5] Melee Attack  with CoolDown
  (Utilities|FlowControl|DoOnce false :!label _label
    (:Completed
      (bind _returnvalue_2 (Collision|SphereTraceForObjects _returnvalue _returnvalue (Variables|Default|GetMeleeAttackRange) (Utilities|Array|MakeArray "ObjectTypeQuery7") false 0 "ForDuration"))
      (if _returnvalue_2
        (Variables|Default|SetCanBite false)
        (Development|PrintString "ChimeraMeleeAttack")
        (Game|Damage|ApplyDamage (Game|GetPlayerCharacter 0) (Variables|Default|GetMeleeAttackDamage) 0 0 "/Game/Blueprints/Combat/BP_BleedDamageType.BP_BleedDamageType_C"))
      (Utilities|FlowControl|Delay (Variables|Default|GetMeleeAttackSpeed))
      (Variables|Default|SetCanBite true)
      (goto _label Reset))))

(event Custom|Rotate
  ;[0.15 0.15 0.15 0.5] Ratating actor toward player
  (Transformation|SetActorRotation (Math|Rotator|FindLookatRotation (Transformation|GetActorLocation) (Transformation|GetActorLocation (Game|GetPlayerCharacter 0)))))

(event Custom|Shoot
  ;[0.15 0.15 0.15 0.5] Range Attack Event with spawning web and reload
  (Utilities|FlowControl|DoOnce false :!label _label
    (:Completed
      (Development|PrintString "ChimeraRangeAttack")
      (Variables|Default|SetCanShoot false)
      (bind _returnvalue (Game|SpawnActorfromClass "/Game/Blueprints/Enemies/Basilisk/BP_VenomSpit.BP_VenomSpit_C" (Transformation|GetWorldTransform (Variables|Default|GetArrow1)) "AlwaysSpawn" "MultiplyWithRoot" 0 0))
      (Game|Damage|ApplyDamage _returnvalue (Variables|Default|GetRangedAttackDamage) 0 0)
      (Utilities|FlowControl|Delay (Variables|Default|GetRangedAttackSpeed))
      (Variables|Default|SetCanShoot true)
      (goto _label Reset))))

(event Custom|Charge
  ;[0.15 0.15 0.15 0.5] Charge Attack with damage and trigger
  (Utilities|FlowControl|DoOnce false :!label _label
    (:Completed
      (Development|PrintString "ChimeraChargeAttack")
      (Variables|/Script/Engine.CharacterMovementComponent|SetMaxWalkSpeed (Variables|Character|GetCharacterMovement) (Variables|Default|GetChargeMovementSpeed))
      (Utilities|FlowControl|Delay (Variables|Default|GetChargeAttackSpeed))
      (Variables|Default|SetCanCharge true)
      (goto _label Reset))))

(event EventBeginPlay
  ;[0.15 0.15 0.15 0.5] PresetVariables
  (Variables|Default|SetMaxHealth (* (Variables|Default|GetMaxHealth) (Variables|Default|GetMultipler)))
  (Variables|Default|SetCurrentHealth (Variables|Default|GetMaxHealth))
  (Variables|/Script/Engine.CharacterMovementComponent|SetMaxWalkSpeed (Variables|Character|GetCharacterMovement) (Variables|Default|GetMovementSpeed))
  (Variables|Default|SetMeleeAttackDamage (* (Variables|Default|GetMeleeAttackDamage) (Variables|Default|GetMultipler)))
  (Variables|Default|SetRangedAttackDamage (* (Variables|Default|GetRangedAttackDamage) (Variables|Default|GetMultipler)))
  (Variables|Default|SetChargeAttackDamage (* (Variables|Default|GetChargeAttackDamage) (Variables|Default|GetMultipler)))
  (bind _asbp_player_character (Utilities|Casting|CastToBP_PlayerCharacter (Game|GetPlayerCharacter 0)))
  (bind _asin_game_hud (Utilities|Casting|CastToInGameHud (Variables|/Game/Blueprints/BP_PlayerCharacter.BP_PlayerCharacter_C|GetHUDRef _asbp_player_character)))
  (bind _output_get (Variables|Default|SetHudRef _asin_game_hud))
  (Default|UpdateBossHealth _output_get (Variables|Default|GetCurrentHealth) (Variables|Default|GetMaxHealth))
  (Default|BossBarVisinility (Variables|Default|GetHudRef)))

(event Game|Damage|EventAnyDamage
  (params (Damage :type Float%20%28single-precision%29) (DamageType :type Damage%20Type%20Object%20Reference) (InstigatedBy :type Controller%20Object%20Reference) (DamageCauser :type Actor%20Object%20Reference))
  ;[0.15 0.15 0.15 0.5] Recieve Damage
  (bind _output_get (Variables|Default|SetCurrentHealth (- (Variables|Default|GetCurrentHealth) Damage)))
  (Default|UpdateBossHealth (Variables|Default|GetHudRef) _output_get (Variables|Default|GetMaxHealth)))

(event EventTick
  (params (DeltaSeconds :type Float%20%28single-precision%29))
  (bind _chimeraaudio (Variables|Default|GetChimeraAudio))
  ;[0.15 0.15 0.15 0.5] Death
  (if (<= (Variables|Default|GetCurrentHealth) 0.0)
    (Variables|Default|SetCanShoot false)
    (Variables|Default|SetCanBite false)
    (Variables|Default|SetCanCharge false)
    (Utilities|FlowControl|DoOnce false
      (:Completed
        (Default|BossBarVisinility (Variables|Default|GetHudRef))
        (Components|Movement|StopMovementImmediately (Variables|Character|GetCharacterMovement))
        (Audio|Components|Audio|SetVolumeMultiplier _chimeraaudio 0.5 :!class /Script/Engine.AudioComponent)
        (Audio|Components|Audio|Play _chimeraaudio 0.0)
        (Utilities|FlowControl|Delay 1.0)
        (Actor|DestroyActor)))))

(fn ConstructionScript)