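; Player controller that links the player character to the combat controller component and opens the game's menus.
; It forwards component added and removed events to BPCCombatController through its calls.
; On BeginPlay it caches the controlled BP_PlayerCharacter and binds a dispatcher that relays component destruction requests to that character.
; The pause input pauses the game, shows the pause widget and mouse, while DisplayMenu opens a separate Pause_Menu widget.
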(event Custom|DestoryPawnComponent_Event
  (params (NewParam :type Actor%20Component%20Object%20Reference))
  (Default|CallDestoryComponent (stale EventBeginPlay _output_get) NewParam))

(event Custom|DisplayMenu
  (CallFunction|DisplayPlayerMenu))

(event Input|EnhancedActionEvents|EnhancedInputActionIA_Pause_Game
  (params (ActionValue :type Boolean) (ElapsedSeconds :type Float%20%28double-precision%29) (TriggeredSeconds :type Float%20%28double-precision%29) (InputAction :type Input%20Action%20Object%20Reference :default "/Game/Blueprints/Widgets/MenUz/IA_Pause_Game.IA_Pause_Game"))
  (:Started
    (Game|SetGamePaused true)
    (bind _returnvalue (UserInterface|CreateWidget "/Game/Blueprints/Widgets/MenUz/Pause_Menu/Pasue_Menue_Ui.Pasue_Menue_Ui_C"))
    (UserInterface|Viewport|AddtoViewport _returnvalue 0)
    (CallFunction|ShowMouse)))

(event EventOnComponentAdded
  (params (NewComponent :type Actor%20Component%20Object%20Reference))
  (Default|CallOnComponentAddedComponent (Variables|Default|GetBPC_CombatController) NewComponent))

(event EventOnComponentRemoved
  (params (RemovedComponent :type Actor%20Component%20Object%20Reference))
  (Default|CallOnComponentRemovedComponent (Variables|Default|GetBPC_CombatController) RemovedComponent))

(event EventBeginPlay
  (bind _asbp_player_character (Utilities|Casting|CastToBP_PlayerCharacter (Pawn|GetControlledPawn)))
  (bind _output_get (Variables|Default|SetControlledCharacter _asbp_player_character))
  (EventDispatchers|BindEventtoDestoryPawnComponent (delegate Custom|DestoryPawnComponent_Event)))

(fn ConstructionScript)

(fn DisplayPlayerMenu
  (bind _returnvalue (UserInterface|CreateWidget "/Game/Blueprints/Widgets/MenUz/Pause_Menu/Pause_Menu.Pause_Menu_C"))
  (bind _output_get (LocalVariables|SetWP%20Player%20Menu _returnvalue))
  (UserInterface|Viewport|AddtoViewport _output_get 0))

(fn DsiplayPauseMenueUI
  (bind _returnvalue (UserInterface|CreateWidget "/Game/Blueprints/Widgets/MenUz/Pause_Menu/Pasue_Menue_Ui.Pasue_Menue_Ui_C"))
  (bind _output_get (Variables|Default|SetWB_Player%20Menu _returnvalue))
  (UserInterface|Viewport|AddtoViewport _output_get 0))