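; BP_Skeleton_Base is a skeleton enemy that tracks health, takes damage and is destroyed when its health runs out.
; On BeginPlay it applies its movement speed, fills health and pushes the values to its WBP_Healthbar_Skeleton widget.
; AnyDamage passes through a DoOnce that resets after a delay, giving immunity frames between hits, then updates health and the bar.
; An ApplyDamage node for attack damage exists but is not wired up.
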(event EventBeginPlay
  ;[0.15 0.15 0.6522 0.5] Setting Movement Speed
  (Variables|/Script/Engine.CharacterMovementComponent|SetMaxWalkSpeed (Variables|Character|GetCharacterMovement) (Variables|Default|GetMovement_Speed))
  ;[0.15 0.04078 0.02858 0.5] Setting Current Health To Max Health
  (Variables|Default|SetCurrent_Health (Variables|Default|GetMax_Health))
  (CallFunction|UpdateHealthbar))

(event Game|Damage|EventAnyDamage
  (params (Damage :type Float%20%28single-precision%29) (DamageType :type Damage%20Type%20Object%20Reference) (InstigatedBy :type Controller%20Object%20Reference) (DamageCauser :type Actor%20Object%20Reference))
  ;[1 1 1 0.5] Immunity Frames
  (Utilities|FlowControl|DoOnce false :!label _label
    (:Completed
      ;[0.15 0.02312 0.03 0.5] Health Logic
      (CallFunction|UpdateCurrentHealth Damage)
      (CallFunction|UpdateHealthbar)
      ;[0.15 0.15 0.15 0.5] Check If Skeleton Is Dead
      (if (<= (Variables|Default|GetCurrent_Health) 0.0)
        (Actor|DestroyActor)
        (else
          ;[1 1 1 0.5] Immunity Frames
          (Utilities|FlowControl|Delay (Variables|Default|GetImmunity_Frames))
          (goto _label Reset))))))

(fn ConstructionScript)

(fn UpdateHealthbar
  (bind _aswbp_healthbar_skeleton (Utilities|Casting|CastToWBP_Healthbar_Skeleton (UserInterface|GetUserWidgetObject (Variables|Default|GetWidget))))
  (bind _output_get (Variables|Default|SetAs%20WBP%20Healthbar%20Skeleton _aswbp_healthbar_skeleton))
  (Variables|/Game/Enemies/Skeletons/WBP_Healthbar_Skeleton.WBP_Healthbar_Skeleton_C|SetCurrent%20Health _output_get (Variables|Default|GetCurrent_Health))
  (Variables|/Game/Enemies/Skeletons/WBP_Healthbar_Skeleton.WBP_Healthbar_Skeleton_C|SetMax%20Health _output_get (Variables|Default|GetMax_Health)))

(fn UpdateCurrentHealth
  (params (Damage :type Float%20%28double-precision%29))
  ;[0.15 0.15 0.15 0.5] Update Current Health
  (Variables|Default|SetCurrent_Health (- (Variables|Default|GetCurrent_Health) Damage)))