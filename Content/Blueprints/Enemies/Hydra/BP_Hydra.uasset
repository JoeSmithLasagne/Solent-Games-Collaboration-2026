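; BP_Hydra is a work-in-progress Hydra enemy with bite, tail, fireball and acid attacks, each currently only printing debug text.
; BeginPlay waits a tick, passes combat, movement and per-attack range and delay stats through elite multiplier helpers, then initializes health and healthbar.
; AnyDamage starts a DoOnce-gated immunity timer, while the health, death and player-damage logic in the event graph is disconnected.
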(event Custom|Acid_Ball
  (Development|PrintText "Acid" true true "(R=1.000000,G=0.919676,B=0.055748,A=1.000000)" 0.1))

(event Custom|Tail_Attack
  (Development|PrintText "Tail" true true "(R=1.000000,G=0.491679,B=0.036456,A=1.000000)" 0.1))

(event Custom|Immunity%20Frames%20Finished
  ;[1 1 1 0.502] Immunity Frames
  (Utilities|FlowControl|DoOnce false) ; enters at Reset
)

(event Custom|Fireball
  (Development|PrintText "Fire" true true "(R=1.000000,G=0.639454,B=0.000000,A=1.000000)" 0.1))

(event Custom|Bite_Attack
  (Development|PrintText "Bite" true true "(R=1.000000,G=0.171047,B=0.000000,A=1.000000)" 0.1))

(event EventBeginPlay
  (Utilities|FlowControl|DelayUntilNextTick)
  ;[0.15 0.15 0.15 0.5] Elites Stat Multiplying
  (CallFunction|BlackboardStats)
  (Variables|Stats|SetMovement_Speed (Utilities|StatMultipliers (Variables|Stats|GetMovement_Speed)))
  (Variables|Stats|SetMax_Health (Utilities|StatMultipliers (Variables|Stats|GetMax_Health)))
  (Variables|Stats|SetAttack_Damage_Bite (Utilities|StatMultipliers (Variables|Stats|GetAttack_Damage_Bite)))
  (Variables|Stats|SetImmunity_Frames_Timer (Utilities|StatMultipliers (Variables|Stats|GetImmunity_Frames_Timer)))
  (Variables|Stats|SetAttack%20Delay (Utilities|TimerMultiplier (Variables|Stats|GetAttack%20Delay)))
  (Variables|Stats|SetAttack%20Range (Utilities|StatMultipliers (Variables|Stats|GetAttack%20Range)))
  ;[0.15 0.15 0.6514 0.502] Setting Movement Speed
  (Variables|/Script/Engine.CharacterMovementComponent|SetMaxWalkSpeed (Variables|Character|GetCharacterMovement) (Variables|Stats|GetMovement_Speed))
  ;[0.15 0.04092 0.02843 0.502] Setting Current Health To Max Health
  (Variables|Stats|SetCurrent_Health (Variables|Stats|GetMax_Health))
  (CallFunction|UpdateHealthbar))

(event Game|Damage|EventAnyDamage
  (params (Damage :type Float%20%28single-precision%29) (DamageType :type Damage%20Type%20Object%20Reference) (InstigatedBy :type Controller%20Object%20Reference) (DamageCauser :type Actor%20Object%20Reference))
  ;[1 1 1 0.502] Immunity Frames
  (Utilities|FlowControl|DoOnce false
    (:Completed
      (Utilities|Time|SetTimerbyFunctionName 0 "Immunity Frames Finished" (Variables|Stats|GetImmunity_Frames_Timer)))))

(fn ConstructionScript)

(fn UpdateHealthbar
  (bind _aswbp_healthbar_skeleton (Utilities|Casting|CastToWBP_Healthbar_Skeleton (UserInterface|GetUserWidgetObject (Variables|Default|GetHealthbar))))
  (bind _output_get (Variables|Default|SetAs%20WBP%20Healthbar%20Skeleton _aswbp_healthbar_skeleton))
  ;[0.15 0.1222 0.05534 0.5] Set helth variables in the healthbar function
  (Variables|/Game/Blueprints/Enemies/Skeletons/WBP_Healthbar_Skeleton.WBP_Healthbar_Skeleton_C|SetCurrent%20Health _output_get (Variables|Stats|GetCurrent_Health))
  (Variables|/Game/Blueprints/Enemies/Skeletons/WBP_Healthbar_Skeleton.WBP_Healthbar_Skeleton_C|SetMax%20Health _output_get (Variables|Stats|GetMax_Health)))

(fn UpdateCurrentHealth
  (params (Damage :type Float%20%28double-precision%29))
  ;[0.15 0.0156 0.004484 0.5] Update Current Health
  (Variables|Stats|SetCurrent_Health (- (Variables|Stats|GetCurrent_Health) Damage)))

(fn BlackboardStats
  (Variables|Blackboard|SetAttack%20Range%20Bite (Utilities|RangeAddon (Utilities|StatMultipliers (Variables|Blackboard|GetAttack%20Range%20Bite))))
  (Variables|Blackboard|SetAttack%20Delay%20Bite (Utilities|StatMultipliers (Variables|Blackboard|GetAttack%20Delay%20Bite)))
  (Variables|Blackboard|SetAttack%20Range%20Tail (Utilities|RangeAddon (Utilities|StatMultipliers (Variables|Blackboard|GetAttack%20Range%20Tail))))
  (Variables|Blackboard|SetAttack%20Delay%20Tail (Utilities|StatMultipliers (Variables|Blackboard|GetAttack%20Delay%20Tail)))
  (Variables|Blackboard|SetAttack%20Range%20Acid (Utilities|RangeAddon (Utilities|StatMultipliers (Variables|Blackboard|GetAttack%20Range%20Acid))))
  (Variables|Blackboard|SetAttack%20Delay%20Acid (Utilities|StatMultipliers (Variables|Blackboard|GetAttack%20Delay%20Acid)))
  (Variables|Blackboard|SetAttack%20Range%20Fireball (Utilities|RangeAddon (Utilities|StatMultipliers (Variables|Blackboard|GetAttack%20Range%20Fireball))))
  (Variables|Blackboard|SetAttack%20Delay%20Fireball (Utilities|StatMultipliers (Variables|Blackboard|GetAttack%20Delay%20Fireball))))