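; Blueprint function library that creates, ticks and removes timed combat hitboxes stored in caller-supplied arrays.
; Createhitbox adds instances; HitboxTick2 box-traces active ones on Visibility relative to their owning actor, deactivates expired ones and removes inactive ones.
; Per-instance parallel arrays track hit actors for re-hit cooldowns, and the tick returns at the first trace hit.
; HitboxTick is a simpler world-space variant; both draw debug traces.
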(fn HitboxTick
  (params (Hitboxes :type Array%20of%20Struct%20Hitbox%20Data%20Structures))
  (bind _returnvalue (Utilities|Time|GetGameTimeinSeconds))
  (Utilities|FlowControl|Sequence
    (:then_0
      (if (> (Utilities|Array|Length Hitboxes) 0)
        (for (_array_element _array_index) Hitboxes
          (if (.Active (Utilities|Struct|BreakStruct_HitboxData _array_element))
            (if (> _returnvalue (+ (.LifeTime (Utilities|Struct|BreakStruct_HitboxData _array_element)) (.StartTime (Utilities|Struct|BreakStruct_HitboxData _array_element))))
              (bind _structout (Utilities|Struct|SetmembersinStruct_HitboxData _array_element false))
              (Utilities|Array|SetArrayElem Hitboxes _array_index _structout true)
              (else
                (bind (_outhit _returnvalue_2) (Collision|BoxTraceByChannel 0 (- (.location (.Transform (Utilities|Struct|BreakStruct_HitboxData _array_element))) (* (Math|Vector|GetForwardVector (.rotation (.Transform (Utilities|Struct|BreakStruct_HitboxData _array_element)))) (/ (.scale (.Transform (Utilities|Struct|BreakStruct_HitboxData _array_element))) 2))) (+ (.location (.Transform (Utilities|Struct|BreakStruct_HitboxData _array_element))) (* (Math|Vector|GetForwardVector (.rotation (.Transform (Utilities|Struct|BreakStruct_HitboxData _array_element)))) (/ (.scale (.Transform (Utilities|Struct|BreakStruct_HitboxData _array_element))) 2))) (Math|Vector|MakeVector 0.0 (.Y (Math|Vector|BreakVector (/ (.scale (.Transform (Utilities|Struct|BreakStruct_HitboxData _array_element))) 2))) (.Z (Math|Vector|BreakVector (/ (.scale (.Transform (Utilities|Struct|BreakStruct_HitboxData _array_element))) 2)))) (.rotation (.Transform (Utilities|Struct|BreakStruct_HitboxData _array_element))) "TraceTypeQuery1" false 0 "ForDuration" true "(R=1.000000,G=0.000000,B=0.000000,A=1.000000)" "(R=0.000000,G=1.000000,B=0.000000,A=1.000000)" _returnvalue))
                (return _outhit _returnvalue_2 _array_element)))
            (else
              (Development|PrintString 0 "Dead")
              (Utilities|Array|RemoveIndex Hitboxes _array_index))))))))

(fn GetHitboxfromKey
  (params (Hitboxes :type Array%20of%20Struct%20Hitbox%20Data%20Structures) (Key :type String))
  (bind _array_element (Utilities|Array|ForEachLoopwithBreak Hitboxes :!label _label)
    (:LoopBody
      (if (Utilities|Enum|Equal(Enum) Key (.Key (Utilities|Struct|BreakStruct_HitboxData _array_element)))
        (Utilities|FlowControl|Sequence
          (:then_0
            (return _array_element (.Key (Utilities|Struct|BreakStruct_HitboxData _array_element)) (Utilities|Enum|Equal(Enum) Key (.Key (Utilities|Struct|BreakStruct_HitboxData _array_element)))))
          (:then_1
            (goto _label Break)))))))

(fn HitboxTick2
  (params (Hitbox%20Array :type Array%20of%20Struct%20Hitbox%20Inst%20Structures))
  (bind _returnvalue (Utilities|Time|GetGameTimeinSeconds))
  (bind _returnvalue_2 (Utilities|Time|GetGameTimeinSeconds))
  (if (> (Utilities|Array|Length Hitbox%20Array) 0)
    (for (_array_element _array_index) Hitbox%20Array
      (LocalVariables|SetCurrrentIndex _array_index)
      (LocalVariables|SetCurrentHitboxInst _array_element)
      (if (.Active (Utilities|Struct|BreakStruct_HitboxData (.Data (Utilities|Struct|BreakStruct_HitboxInst _array_element))))
        (if (and (< _returnvalue (+ (.LifeTime (Utilities|Struct|BreakStruct_HitboxData (.Data (Utilities|Struct|BreakStruct_HitboxInst _array_element)))) (.StartTime (Utilities|Struct|BreakStruct_HitboxData (.Data (Utilities|Struct|BreakStruct_HitboxInst _array_element)))))) (> _returnvalue (.StartTime (Utilities|Struct|BreakStruct_HitboxData (.Data (Utilities|Struct|BreakStruct_HitboxInst _array_element))))))
          (Utilities|FlowControl|Sequence
            (:then_0
              (Utilities|Array|Clear (LocalVariables|GetActorsToRemove))
              (LocalVariables|SetTempNameArray (.ActorNames (Utilities|Struct|BreakStruct_HitboxInst (LocalVariables|GetCurrentHitboxInst))))
              (LocalVariables|SetTempActorArray (.HitActors (Utilities|Struct|BreakStruct_HitboxInst (LocalVariables|GetCurrentHitboxInst))))
              (LocalVariables|SetTempTimeArray (.LastCooldownTimes (Utilities|Struct|BreakStruct_HitboxInst (LocalVariables|GetCurrentHitboxInst))))
              (for (_array_element_2 _array_index_2) (LocalVariables|GetTempNameArray)
                (if (<= (+ (Utilities|Array|Get(acopy) (LocalVariables|GetTempTimeArray) _array_index_2) (.HitCooldown (Utilities|Struct|BreakStruct_HitboxData (.Data (Utilities|Struct|BreakStruct_HitboxInst (LocalVariables|GetCurrentHitboxInst)))))) (Utilities|Time|GetGameTimeinSeconds))
                  (Utilities|Array|Add (LocalVariables|GetActorsToRemove) _array_element_2)))
              (for _array_element_3 (LocalVariables|GetActorsToRemove)
                (Utilities|Array|RemoveIndex (LocalVariables|GetTempTimeArray) (Utilities|Array|FindItem (LocalVariables|GetTempNameArray) _array_element_3))
                (Utilities|Array|RemoveIndex (LocalVariables|GetTempActorArray) (Utilities|Array|FindItem (LocalVariables|GetTempNameArray) _array_element_3))
                (Utilities|Array|RemoveIndex (LocalVariables|GetTempNameArray) (Utilities|Array|FindItem (LocalVariables|GetTempNameArray) _array_element_3))
                (bind _structout (Utilities|Struct|SetmembersinStruct_HitboxInst (LocalVariables|GetCurrentHitboxInst) (LocalVariables|GetTempActorArray) (LocalVariables|GetTempNameArray) (LocalVariables|GetTempTimeArray)))
                (Utilities|Array|SetArrayElem Hitbox%20Array (LocalVariables|GetCurrrentIndex) _structout true)))
            (:then_1
              (if (< (.LastUpdate (Utilities|Struct|BreakStruct_HitboxInst (LocalVariables|GetCurrentHitboxInst))) _returnvalue_2)
                (bind _structout_2 (Utilities|Struct|SetmembersinStruct_HitboxInst (LocalVariables|GetCurrentHitboxInst) (+ (.UpdateRate (Utilities|Struct|BreakStruct_HitboxData (.Data (Utilities|Struct|BreakStruct_HitboxInst (LocalVariables|GetCurrentHitboxInst))))) _returnvalue_2)))
                (LocalVariables|SetCurrentHitboxInst _structout_2)
                (bind (_outhit _returnvalue_3) (Collision|BoxTraceByChannel 0 (+ (+ (+ (* (.X (Math|Vector|BreakVector (.location (.Transform (Utilities|Struct|BreakStruct_HitboxData (.Data (Utilities|Struct|BreakStruct_HitboxInst (LocalVariables|GetCurrentHitboxInst)))))))) (Math|Vector|GetForwardVector (Class|KismetMathLibrary|QuatRotator (* (Math|Conversions|ToQuaternion(Rotator) (.rotation (Transformation|GetActorTransform (.Owning_Actor (Utilities|Struct|BreakStruct_HitboxData (.Data (Utilities|Struct|BreakStruct_HitboxInst (LocalVariables|GetCurrentHitboxInst)))))))) (Math|Conversions|ToQuaternion(Rotator) (.rotation (.Transform (Utilities|Struct|BreakStruct_HitboxData (.Data (Utilities|Struct|BreakStruct_HitboxInst (LocalVariables|GetCurrentHitboxInst))))))))))) (* (.Y (Math|Vector|BreakVector (.location (.Transform (Utilities|Struct|BreakStruct_HitboxData (.Data (Utilities|Struct|BreakStruct_HitboxInst (LocalVariables|GetCurrentHitboxInst)))))))) (Math|Vector|GetRightVector (Class|KismetMathLibrary|QuatRotator (* (Math|Conversions|ToQuaternion(Rotator) (.rotation (Transformation|GetActorTransform (.Owning_Actor (Utilities|Struct|BreakStruct_HitboxData (.Data (Utilities|Struct|BreakStruct_HitboxInst (LocalVariables|GetCurrentHitboxInst)))))))) (Math|Conversions|ToQuaternion(Rotator) (.rotation (.Transform (Utilities|Struct|BreakStruct_HitboxData (.Data (Utilities|Struct|BreakStruct_HitboxInst (LocalVariables|GetCurrentHitboxInst))))))))))) (* (.Z (Math|Vector|BreakVector (.location (.Transform (Utilities|Struct|BreakStruct_HitboxData (.Data (Utilities|Struct|BreakStruct_HitboxInst (LocalVariables|GetCurrentHitboxInst)))))))) (Math|Vector|GetUpVector (Class|KismetMathLibrary|QuatRotator (* (Math|Conversions|ToQuaternion(Rotator) (.rotation (Transformation|GetActorTransform (.Owning_Actor (Utilities|Struct|BreakStruct_HitboxData (.Data (Utilities|Struct|BreakStruct_HitboxInst (LocalVariables|GetCurrentHitboxInst)))))))) (Math|Conversions|ToQuaternion(Rotator) (.rotation (.Transform (Utilities|Struct|BreakStruct_HitboxData (.Data (Utilities|Struct|BreakStruct_HitboxInst (LocalVariables|GetCurrentHitboxInst)))))))))))) (.location (Transformation|GetActorTransform (.Owning_Actor (Utilities|Struct|BreakStruct_HitboxData (.Data (Utilities|Struct|BreakStruct_HitboxInst (LocalVariables|GetCurrentHitboxInst)))))))) (* (* (Math|Vector|GetForwardVector (Class|KismetMathLibrary|QuatRotator (* (Math|Conversions|ToQuaternion(Rotator) (.rotation (Transformation|GetActorTransform (.Owning_Actor (Utilities|Struct|BreakStruct_HitboxData (.Data (Utilities|Struct|BreakStruct_HitboxInst (LocalVariables|GetCurrentHitboxInst)))))))) (Math|Conversions|ToQuaternion(Rotator) (.rotation (.Transform (Utilities|Struct|BreakStruct_HitboxData (.Data (Utilities|Struct|BreakStruct_HitboxInst (LocalVariables|GetCurrentHitboxInst)))))))))) (/ (.X (Math|Vector|BreakVector (.scale (.Transform (Utilities|Struct|BreakStruct_HitboxData (.Data (Utilities|Struct|BreakStruct_HitboxInst (LocalVariables|GetCurrentHitboxInst)))))))) 2.0)) -1.0)) (+ (+ (+ (* (.X (Math|Vector|BreakVector (.location (.Transform (Utilities|Struct|BreakStruct_HitboxData (.Data (Utilities|Struct|BreakStruct_HitboxInst (LocalVariables|GetCurrentHitboxInst)))))))) (Math|Vector|GetForwardVector (Class|KismetMathLibrary|QuatRotator (* (Math|Conversions|ToQuaternion(Rotator) (.rotation (Transformation|GetActorTransform (.Owning_Actor (Utilities|Struct|BreakStruct_HitboxData (.Data (Utilities|Struct|BreakStruct_HitboxInst (LocalVariables|GetCurrentHitboxInst)))))))) (Math|Conversions|ToQuaternion(Rotator) (.rotation (.Transform (Utilities|Struct|BreakStruct_HitboxData (.Data (Utilities|Struct|BreakStruct_HitboxInst (LocalVariables|GetCurrentHitboxInst))))))))))) (* (.Y (Math|Vector|BreakVector (.location (.Transform (Utilities|Struct|BreakStruct_HitboxData (.Data (Utilities|Struct|BreakStruct_HitboxInst (LocalVariables|GetCurrentHitboxInst)))))))) (Math|Vector|GetRightVector (Class|KismetMathLibrary|QuatRotator (* (Math|Conversions|ToQuaternion(Rotator) (.rotation (Transformation|GetActorTransform (.Owning_Actor (Utilities|Struct|BreakStruct_HitboxData (.Data (Utilities|Struct|BreakStruct_HitboxInst (LocalVariables|GetCurrentHitboxInst)))))))) (Math|Conversions|ToQuaternion(Rotator) (.rotation (.Transform (Utilities|Struct|BreakStruct_HitboxData (.Data (Utilities|Struct|BreakStruct_HitboxInst (LocalVariables|GetCurrentHitboxInst))))))))))) (* (.Z (Math|Vector|BreakVector (.location (.Transform (Utilities|Struct|BreakStruct_HitboxData (.Data (Utilities|Struct|BreakStruct_HitboxInst (LocalVariables|GetCurrentHitboxInst)))))))) (Math|Vector|GetUpVector (Class|KismetMathLibrary|QuatRotator (* (Math|Conversions|ToQuaternion(Rotator) (.rotation (Transformation|GetActorTransform (.Owning_Actor (Utilities|Struct|BreakStruct_HitboxData (.Data (Utilities|Struct|BreakStruct_HitboxInst (LocalVariables|GetCurrentHitboxInst)))))))) (Math|Conversions|ToQuaternion(Rotator) (.rotation (.Transform (Utilities|Struct|BreakStruct_HitboxData (.Data (Utilities|Struct|BreakStruct_HitboxInst (LocalVariables|GetCurrentHitboxInst)))))))))))) (.location (Transformation|GetActorTransform (.Owning_Actor (Utilities|Struct|BreakStruct_HitboxData (.Data (Utilities|Struct|BreakStruct_HitboxInst (LocalVariables|GetCurrentHitboxInst)))))))) (* (Math|Vector|GetForwardVector (Class|KismetMathLibrary|QuatRotator (* (Math|Conversions|ToQuaternion(Rotator) (.rotation (Transformation|GetActorTransform (.Owning_Actor (Utilities|Struct|BreakStruct_HitboxData (.Data (Utilities|Struct|BreakStruct_HitboxInst (LocalVariables|GetCurrentHitboxInst)))))))) (Math|Conversions|ToQuaternion(Rotator) (.rotation (.Transform (Utilities|Struct|BreakStruct_HitboxData (.Data (Utilities|Struct|BreakStruct_HitboxInst (LocalVariables|GetCurrentHitboxInst)))))))))) (/ (.X (Math|Vector|BreakVector (.scale (.Transform (Utilities|Struct|BreakStruct_HitboxData (.Data (Utilities|Struct|BreakStruct_HitboxInst (LocalVariables|GetCurrentHitboxInst)))))))) 2.0))) (Math|Vector|MakeVector (* (/ (.X (Math|Vector|BreakVector (.scale (.Transform (Utilities|Struct|BreakStruct_HitboxData (.Data (Utilities|Struct|BreakStruct_HitboxInst (LocalVariables|GetCurrentHitboxInst)))))))) 2.0) 0.0) (.Y (Math|Vector|BreakVector (.scale (.Transform (Utilities|Struct|BreakStruct_HitboxData (.Data (Utilities|Struct|BreakStruct_HitboxInst (LocalVariables|GetCurrentHitboxInst)))))))) (.Z (Math|Vector|BreakVector (.scale (.Transform (Utilities|Struct|BreakStruct_HitboxData (.Data (Utilities|Struct|BreakStruct_HitboxInst (LocalVariables|GetCurrentHitboxInst))))))))) (Class|KismetMathLibrary|QuatRotator (* (Math|Conversions|ToQuaternion(Rotator) (.rotation (Transformation|GetActorTransform (.Owning_Actor (Utilities|Struct|BreakStruct_HitboxData (.Data (Utilities|Struct|BreakStruct_HitboxInst (LocalVariables|GetCurrentHitboxInst)))))))) (Math|Conversions|ToQuaternion(Rotator) (.rotation (.Transform (Utilities|Struct|BreakStruct_HitboxData (.Data (Utilities|Struct|BreakStruct_HitboxInst (LocalVariables|GetCurrentHitboxInst))))))))) "TraceTypeQuery1" false (Utilities|Array|MakeArray (.Owning_Actor (Utilities|Struct|BreakStruct_HitboxData (.Data (Utilities|Struct|BreakStruct_HitboxInst (LocalVariables|GetCurrentHitboxInst)))))) "ForDuration" true "(R=1.000000,G=0.000000,B=0.000000,A=1.000000)" "(R=0.000000,G=1.000000,B=0.000000,A=1.000000)" (.UpdateRate (Utilities|Struct|BreakStruct_HitboxData (.Data (Utilities|Struct|BreakStruct_HitboxInst (LocalVariables|GetCurrentHitboxInst)))))))
                (bind _output_get (LocalVariables|SetHitResult _outhit))
                (if _returnvalue_3
                  (if (!= (Utilities|Array|FindItem (.HitActors (Utilities|Struct|BreakStruct_HitboxInst (LocalVariables|GetCurrentHitboxInst))) (.HitActor (Collision|BreakHitResult _output_get))) -1)
                    (return 0 true "" "")
                    (else
                      (Development|PrintString 0 (Utilities|GetDisplayName (.HitActor (Collision|BreakHitResult _output_get))) true true "(R=1.000000,G=0.000000,B=0.737911,A=1.000000)")
                      (LocalVariables|SetTempActorArray (.HitActors (Utilities|Struct|BreakStruct_HitboxInst (LocalVariables|GetCurrentHitboxInst))))
                      (LocalVariables|SetTempNameArray (.ActorNames (Utilities|Struct|BreakStruct_HitboxInst (LocalVariables|GetCurrentHitboxInst))))
                      (LocalVariables|SetTempTimeArray (.LastCooldownTimes (Utilities|Struct|BreakStruct_HitboxInst (LocalVariables|GetCurrentHitboxInst))))
                      (bind _returnvalue_4 (Utilities|Array|AddUnique (LocalVariables|GetTempActorArray) (.HitActor (Collision|BreakHitResult (LocalVariables|GetHitResult)))))
                      (Utilities|Array|Insert (LocalVariables|GetTempNameArray) (Utilities|GetDisplayName (.HitActor (Collision|BreakHitResult (LocalVariables|GetHitResult)))) _returnvalue_4)
                      (Utilities|Array|Insert (LocalVariables|GetTempTimeArray) (Utilities|Time|GetGameTimeinSeconds) _returnvalue_4)
                      (bind _structout_3 (Utilities|Struct|SetmembersinStruct_HitboxInst (LocalVariables|GetCurrentHitboxInst) (LocalVariables|GetTempActorArray) (LocalVariables|GetTempNameArray) (LocalVariables|GetTempTimeArray)))
                      (Utilities|Array|SetArrayElem Hitbox%20Array (LocalVariables|GetCurrrentIndex) _structout_3 true)
                      (return (.CallingComponent (Utilities|Struct|BreakStruct_HitboxInst (LocalVariables|GetCurrentHitboxInst))) true (LocalVariables|GetHitResult) (LocalVariables|GetCurrentHitboxInst))))))))
          (elif (<= (+ (.LifeTime (Utilities|Struct|BreakStruct_HitboxData (.Data (Utilities|Struct|BreakStruct_HitboxInst _array_element)))) (.StartTime (Utilities|Struct|BreakStruct_HitboxData (.Data (Utilities|Struct|BreakStruct_HitboxInst _array_element))))) _returnvalue)
            (bind _structout_4 (Utilities|Struct|SetmembersinStruct_HitboxData (.Data (Utilities|Struct|BreakStruct_HitboxInst (LocalVariables|GetCurrentHitboxInst))) false))
            (bind _structout_5 (Utilities|Struct|SetmembersinStruct_HitboxInst (LocalVariables|GetCurrentHitboxInst) _structout_4))
            (Utilities|Array|SetArrayElem Hitbox%20Array 0 _structout_5 true)))
        (else
          (CallFunction|RemoveHitbox Hitbox%20Array (LocalVariables|GetCurrentHitboxInst)))))
    (return 0 false "" "")))

(fn RemoveHitbox
  (params (Hitbox%20Array :type Array%20of%20Struct%20Hitbox%20Inst%20Structures) (Hitbox :type Struct%20Hitbox%20Inst%20Structure))
  (Utilities|Array|RemoveItem Hitbox%20Array Hitbox)
  (return))

(fn Createhitbox
  (params (hitbox%20array :type Array%20of%20Struct%20Hitbox%20Inst%20Structures) (hitbox%20data :type Struct%20Hitbox%20Data%20Structure) (Calling%20Component :type Actor%20Component%20Object%20Reference))
  (Development|PrintString 0 (Utilities|GetDisplayName Calling%20Component) true true "(R=0.057687,G=1.000000,B=0.001574,A=1.000000)")
  (Utilities|Array|Add hitbox%20array (Utilities|Struct|MakeStruct_HitboxInst hitbox%20data Calling%20Component))
  (Development|PrintString 0 "HitboxAdded" true true "(R=1.000000,G=0.000000,B=0.737911,A=1.000000)"))