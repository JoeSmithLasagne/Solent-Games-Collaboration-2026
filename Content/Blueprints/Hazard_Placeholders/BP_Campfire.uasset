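; BP_Campfire is a placeholder hazard that repeatedly damages the player while they overlap its DamageTrigger.
; Tick runs through a DoOnce, scans the trigger for the player character and applies Damage when it finds player 0.
; A Retrigger event resets the gate after DamageRate seconds following a hit, or on the next tick when nothing was damaged, so polling doubles as the damage cooldown.
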(event Custom|Retrigger
  (bind _returnvalue (Game|GetPlayerCharacter 0))
  (Utilities|FlowControl|DoOnce false) ; enters at Reset
)

(event EventBeginPlay)

(event Collision|EventActorBeginOverlap
  (params (OtherActor :type Actor%20Object%20Reference)))

(event EventTick
  (params (DeltaSeconds :type Float%20%28single-precision%29))
  (bind _returnvalue (Game|GetPlayerCharacter 0))
  (Utilities|FlowControl|DoOnce false
    (:Completed
      (Variables|Logic|SetDamage%20Applied false)
      (for _array_element (Collision|GetOverlappingActors (Variables|Default|GetDamage%20Trigger) "/Game/Blueprints/BP_PlayerCharacter.BP_PlayerCharacter_C" :!class /Script/Engine.PrimitiveComponent)
        (if (== _array_element _returnvalue)
          (Variables|Logic|SetDamage%20Applied true)
          (Game|Damage|ApplyDamage _returnvalue (Variables|Stats|GetDamage) 0 0)
          (Utilities|FlowControl|Delay (Variables|Stats|GetDamage%20rate))
          (CallFunction|Retrigger)))
      (Utilities|FlowControl|DelayUntilNextTick)
      (if (not (Variables|Logic|GetDamage%20Applied))
        (CallFunction|Retrigger)))))

(fn ConstructionScript)