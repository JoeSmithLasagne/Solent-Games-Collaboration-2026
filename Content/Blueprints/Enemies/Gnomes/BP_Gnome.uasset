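; Gnome enemy character that damages the player and can be killed, with health shown on a widget healthbar.
; Attack applies placeholder damage directly to player 0, counting hits and blocking further attacks during a cooldown once the limit is reached.
; Incoming damage passes through a DoOnce gate, reset by timer for immunity frames, then lowers health and either refreshes the healthbar or destroys the gnome.
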(event Custom|Attack
  (if (not (>= (Variables|Default|GetCurrent%20Attack) (Variables|Stats|GetAttacks%20before%20cooldown)))
    ;[0.15 0 0.01939 0.5] Temporary damage
    (Game|Damage|ApplyDamage (Game|GetPlayerCharacter 0) (Variables|Stats|GetAttack%20Damage) 0 0)
    ;[0 0.5323 0.0222 0.5] Increment attacks by 1
    (Variables|Default|SetCurrent%20Attack (+ (Variables|Default|GetCurrent%20Attack) 1))
    ;[0.1031 0 0.008199 0.5] Check if on last attack
    (if (>= (Variables|Default|GetCurrent%20Attack) (Variables|Stats|GetAttacks%20before%20cooldown))
      ;[0.15 0.15 0.15 0.5] Last attack cooldown
      (Utilities|FlowControl|Delay (Variables|Stats|GetFinal%20Attack%20Cooldown))
      (Variables|Default|SetCurrent%20Attack 0))))

(event Custom|Immunity%20frames%20done
  ;[1 1 1 0.502] Immunity Frames
  (Utilities|FlowControl|DoOnce false) ; enters at Reset
)

(event EventBeginPlay
  ;[0.15 0.15 0.6514 0.502] Setting Movement Speed
  (Variables|/Script/Engine.CharacterMovementComponent|SetMaxWalkSpeed (Variables|Character|GetCharacterMovement) (Variables|Stats|GetMovement%20Speed))
  ;[0.15 0.04092 0.02843 0.502] Setting Current Health To Max Health
  (Variables|Stats|SetCurrent%20Health (Variables|Stats|GetMax%20Health))
  (CallFunction|UpdateHealthbar))

(event Game|Damage|EventAnyDamage
  (params (Damage :type Float%20%28single-precision%29) (DamageType :type Damage%20Type%20Object%20Reference) (InstigatedBy :type Controller%20Object%20Reference) (DamageCauser :type Actor%20Object%20Reference))
  ;[1 1 1 0.502] Immunity Frames
  (Utilities|FlowControl|DoOnce false
    (:Completed
      (Utilities|Time|SetTimerbyFunctionName 0 "Immunity frames done" (Variables|Stats|GetImmunity%20Frames))
      (CallFunction|UpdateCurrentHealth Damage)
      ;[0.15 0.07087 0.05015 0.5] Check if the gnome is dead
      (if (<= (Variables|Stats|GetCurrent%20Health) 0.0)
        (Actor|DestroyActor)
        (else
          (CallFunction|UpdateHealthbar))))))

(fn ConstructionScript)

(fn UpdateHealthbar
  (bind _aswbp_healthbar_skeleton (Utilities|Casting|CastToWBP_Healthbar_Skeleton (UserInterface|GetUserWidgetObject (Variables|Default|GetHealthbar))))
  ;[0.15 0.1222 0.05534 0.5] Set helth variables in the healthbar function
  (Variables|/Game/Blueprints/Enemies/Skeletons/WBP_Healthbar_Skeleton.WBP_Healthbar_Skeleton_C|SetCurrent%20Health _aswbp_healthbar_skeleton (Variables|Stats|GetCurrent%20Health))
  (Variables|/Game/Blueprints/Enemies/Skeletons/WBP_Healthbar_Skeleton.WBP_Healthbar_Skeleton_C|SetMax%20Health _aswbp_healthbar_skeleton (Variables|Stats|GetMax%20Health)))

(fn UpdateCurrentHealth
  (params (Damage :type Float%20%28double-precision%29))
  ;[0.15 0.0156 0.004484 0.5] Update Current Health
  (Variables|Stats|SetCurrent%20Health (- (Variables|Stats|GetCurrent%20Health) Damage)))