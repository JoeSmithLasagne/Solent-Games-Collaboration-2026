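; Base spider enemy with health, a ranged web attack and a venomous melee bite, with health and damage scaled by a multiplier.
; Custom events face the player, spawn web projectiles or sphere-trace before biting, with both attacks cooldown-gated by DoOnce and delays.
; Projectile damage is passed by applying damage to the spawned projectile itself.
; Received damage updates the health bar widget, while Tick detects zero health, stops movement, plays audio and destroys the spider.
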(event Custom|Shoot
  ;[0.15 0.15 0.15 0.5] Range Attack Event with spawning web and reload
  (Utilities|FlowControl|DoOnce false :!label _label
    (:Completed
      (Development|PrintString "SpiderRangeAttack")
      (Variables|Default|SetCanShoot false)
      (bind _returnvalue (Game|SpawnActorfromClass "/Game/Blueprints/Enemies/Spider/BP_WebProjectile.BP_WebProjectile_C" (Transformation|GetWorldTransform (Variables|Default|GetSphere2)) "AlwaysSpawn" "MultiplyWithRoot" 0 0))
      (Game|Damage|ApplyDamage _returnvalue (Variables|Default|GetProjectileDamage) 0 self)
      (Utilities|FlowControl|Delay (Variables|Default|GetProjectileAttackSpeed))
      (Variables|Default|SetCanShoot true)
      (goto _label Reset))))

(event Custom|Attack
  (bind _arrow1 (Variables|Default|GetArrow1))
  (bind _returnvalue (Transformation|GetWorldLocation _arrow1))
  ;[0.15 0.15 0.15 0.5] Melee Attack  with CoolDown
  (Utilities|FlowControl|DoOnce false :!label _label
    (:Completed
      (bind _returnvalue_2 (Collision|SphereTraceForObjects _returnvalue _returnvalue (Variables|Default|GetAttackRange) (Utilities|Array|MakeArray "ObjectTypeQuery7") false 0 "ForDuration"))
      (if _returnvalue_2
        (Variables|Default|SetCanBite false)
        (Development|PrintString "SpiderMeleeAttack")
        (Game|Damage|ApplyDamage (Game|GetPlayerCharacter 0) (Variables|Default|GetMeleeAttackDamage) 0 0 "/Game/Blueprints/Combat/BP_VenomDamageType.BP_VenomDamageType_C"))
      (Utilities|FlowControl|Delay (Variables|Default|GetMeleeAttackSpeed))
      (Variables|Default|SetCanBite true)
      (goto _label Reset))))

(event Custom|Rotate
  ;[0.15 0.15 0.15 0.5] Ratating actor toward player
  (Transformation|SetActorRotation (Math|Rotator|FindLookatRotation (Transformation|GetActorLocation) (Transformation|GetActorLocation (Game|GetPlayerCharacter 0)))))

(event Custom|UpdateHealthBar
  ;[0.15 0.15 0.15 0.5] HealthBar
  (bind _aswbp_healthbar_skeleton (Utilities|Casting|CastToWBP_Healthbar_Skeleton (UserInterface|GetUserWidgetObject (Variables|Default|GetHealthBar))))
  ;[0.15 0.1222 0.05534 0.5] Set helth variables in the healthbar function
  (Variables|/Game/Blueprints/Enemies/Skeletons/WBP_Healthbar_Skeleton.WBP_Healthbar_Skeleton_C|SetCurrent%20Health _aswbp_healthbar_skeleton (Variables|Default|GetCurrentHealth))
  (Variables|/Game/Blueprints/Enemies/Skeletons/WBP_Healthbar_Skeleton.WBP_Healthbar_Skeleton_C|SetMax%20Health _aswbp_healthbar_skeleton (Variables|Default|GetMaxHealth)))

(event EventBeginPlay
  ;[0.15 0.15 0.15 0.5] PresetVariables
  (Variables|Default|SetMaxHealth (* (Variables|Default|GetMaxHealth) (Variables|Default|GetMultipler)))
  (Variables|Default|SetCurrentHealth (Variables|Default|GetMaxHealth))
  (Variables|/Script/Engine.CharacterMovementComponent|SetMaxWalkSpeed (Variables|Character|GetCharacterMovement) (Variables|Default|GetMovementSpeed))
  (Variables|Default|SetMeleeAttackDamage (* (Variables|Default|GetMeleeAttackDamage) (Variables|Default|GetMultipler)))
  (Variables|Default|SetProjectileDamage (* (Variables|Default|GetProjectileDamage) (Variables|Default|GetMultipler)))
  (CallFunction|UpdateHealthBar))

(event Game|Damage|EventAnyDamage
  (params (Damage :type Float%20%28single-precision%29) (DamageType :type Damage%20Type%20Object%20Reference) (InstigatedBy :type Controller%20Object%20Reference) (DamageCauser :type Actor%20Object%20Reference))
  ;[0.15 0.15 0.15 0.5] Recieve Damage
  (Variables|Default|SetCurrentHealth (- (Variables|Default|GetCurrentHealth) Damage))
  (CallFunction|UpdateHealthBar))

(event EventTick
  (params (DeltaSeconds :type Float%20%28single-precision%29))
  (bind _spideraudio (Variables|Default|GetSpiderAudio))
  ;[0.15 0.15 0.15 0.5] Death
  (if (<= (Variables|Default|GetCurrentHealth) 0.0)
    (Variables|Default|SetCanShoot false)
    (Variables|Default|SetCanBite false)
    (Utilities|FlowControl|DoOnce false
      (:Completed
        (Components|Movement|StopMovementImmediately (Variables|Character|GetCharacterMovement))
        (Audio|Components|Audio|SetVolumeMultiplier _spideraudio 0.5 :!class /Script/Engine.AudioComponent)
        (Audio|Components|Audio|Play _spideraudio 0.0)
        (Utilities|FlowControl|Delay 1.0)
        (Actor|DestroyActor)))))

(fn ConstructionScript)